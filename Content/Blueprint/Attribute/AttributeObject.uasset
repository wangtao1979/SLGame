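; Attribute container object that stores one numeric value per attribute enum entry in an array indexed by enum value.
; It offers per-type get and set plus element-wise clear, add, copy and subtract, where Sub yields source minus own value.
; ComputeBuff overwrites each value with (base + flat buff) × (1 + percent buff), taken from two other attribute sets.
; Load restores the array from serialized data, then resizes it to the enum count.
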(fn `add`
  (params (src :type "/Game/Blueprint/Attribute/AttributeObject Object Reference"))
  (bind _data (`self.data`))
  ;[1 1 1] 把2个属性相加
  (for (_array_element _array_index) (`self.get_all` src)
    (`KismetArrayLibrary.Array_Set` _data _array_index (+ _array_element (`KismetArrayLibrary.Array_Get` _data _array_index)) true)))

(fn `clear`
  (bind _data (`self.data`))
  ;[1 1 1] 把属性全部设置为0
  (for _index (range (+ (`KismetArrayLibrary.Array_LastIndex` _data) 1))
    (`KismetArrayLibrary.Array_Set` _data _index)))

(fn `compute`
  (params (init :type "Float (double-precision)") (buff :type "Float (double-precision)") (buff_per :type "Float (double-precision)"))
  (returns (value :type "Float (double-precision)"))
  ;[1 1 1] 进行加成属性计算
  (return (* (+ init buff) (+ buff_per 1.0))))

(fn `compute_buff`
  (params (buff :type "/Game/Blueprint/Attribute/AttributeObject Object Reference") (buff_per :type "/Game/Blueprint/Attribute/AttributeObject Object Reference"))
  ;[1 1 1] 重新计算整个属性
  (for (_array_element _array_index) (`self.data`)
    (`KismetArrayLibrary.Array_Set` (`self.data`) _array_index (`self.compute` _array_element (`KismetArrayLibrary.Array_Get` (`self.get_all` buff) _array_index) (`KismetArrayLibrary.Array_Get` (`self.get_all` buff_per) _array_index)))))

(fn `copy`
  (params (src :type "/Game/Blueprint/Attribute/AttributeObject Object Reference"))
  ;[1 1 1] 复制一个属性值
  (for (_array_element _array_index) (`self.get_all` src)
    (`KismetArrayLibrary.Array_Set` (`self.data`) _array_index _array_element true)))

(fn `get`
  (params (type :type "/Game/Blueprint/Attribute/AttributeDefine Enum"))
  (returns (value :type "Float (double-precision)"))
  ;[1 1 1] 获取某个属性
  (return (`KismetArrayLibrary.Array_Get` (`self.data`) (`KismetMathLibrary.Conv_ByteToInt` type))))

(fn `get_all`
  (returns (data :type "Array of Float (double-precision)"))
  ;[1 1 1] 获取属性数组
  (return (`self.data`)))

(fn `init`
  ;[1 1 1] 根据属性值初始化属性列表
  (`KismetArrayLibrary.Array_Resize` (`self.data`) (enumcount `/Game/Blueprint/Attribute/AttributeDefine`)))

(fn `load`
  (params (data :type "/Game/Blueprint/Attribute/AttributeData Structure"))
  (bind _output_get (set `self.SerializationData` data))
  (set `self.data` (`.data_3_E4E8807D41D000094D5FE68429D9B32B` (break `/Game/Blueprint/Attribute/AttributeData` _output_get)))
  (`self.init`))

(fn `set`
  (params (type :type "/Game/Blueprint/Attribute/AttributeDefine Enum") (value :type "Float (double-precision)"))
  ;[1 1 1] 设置某个单独属性
  (`KismetArrayLibrary.Array_Set` (`self.data`) (`KismetMathLibrary.Conv_ByteToInt` type) value true))

(fn `sub`
  (params (src :type "/Game/Blueprint/Attribute/AttributeObject Object Reference"))
  (bind _data (`self.data`))
  ;[1 1 1] 把2个属性相减
  (for (_array_element _array_index) (`self.get_all` src)
    (`KismetArrayLibrary.Array_Set` _data _array_index (- _array_element (`KismetArrayLibrary.Array_Get` _data _array_index)) true)))