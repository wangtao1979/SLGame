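; Attribute buff container that holds a list of buffs and computes the resulting attribute set.
; Init constructs three AttributeObjects: the final attributes, additive buff totals and percentage buff totals.
; Compute resets all three, copying an optional base into the final set, lets each active buff accumulate into both totals, then applies them through ComputeBuff.
; Adding, removing or clearing buffs only edits the list, without recomputing.
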(fn `add`
  (params (buff :type "/Game/Blueprint/Attribute/AttributeBuff Object Reference"))
  ;[1 1 1] 添加BUFF
  (`KismetArrayLibrary.Array_Add` (`self.buff_list`) buff))

(fn `clear`
  (`KismetArrayLibrary.Array_Clear` (`self.buff_list`)))

(fn `compute`
  (params (init :type "/Game/Blueprint/Attribute/AttributeObject Object Reference"))
  (returns (attribute :type "/Game/Blueprint/Attribute/AttributeObject Object Reference"))
  ;[1 1 1] 重新计算所有的属性
  (`/Engine/EditorBlueprintResources/StandardMacros.IsValid` init
    (:`Is Valid`
      (`/Game/Blueprint/Attribute/AttributeObject.copy` (`self.attribute`) init))
    (:`Is Not Valid`
      (`/Game/Blueprint/Attribute/AttributeObject.clear` (`self.attribute`))))
  (`/Game/Blueprint/Attribute/AttributeObject.clear` (`self.buff`))
  (`/Game/Blueprint/Attribute/AttributeObject.clear` (`self.buffer_per`))
  (for _array_element (`self.buff_list`)
    (if (`/Game/Blueprint/Attribute/AttributeBuff.is_active` _array_element 0)
      (`/Game/Blueprint/Attribute/AttributeBuff.count` _array_element (`self.buff`) (`self.buffer_per`))))
  (`/Game/Blueprint/Attribute/AttributeObject.compute_buff` (`self.attribute`) (`self.buff`) (`self.buffer_per`))
  (return (`self.attribute`)))

(fn `get_attribute`
  (returns (attribute :type "/Game/Blueprint/Attribute/AttributeObject Object Reference"))
  (return (`self.attribute`)))

(fn `init`
  ;[1 1 1] 初始化
  (`|ExecutionSequence`
    (:`then_0`
      (bind _returnvalue (`|GenericCreateObject` "/Game/Blueprint/Attribute/AttributeObject.AttributeObject_C" self))
      (bind _output_get (set `self.attribute` _returnvalue))
      (`/Game/Blueprint/Attribute/AttributeObject.init` _output_get))
    (:`then_1`
      (bind _returnvalue_2 (`|GenericCreateObject` "/Game/Blueprint/Attribute/AttributeObject.AttributeObject_C" self))
      (bind _output_get_2 (set `self.buffer_per` _returnvalue_2))
      (`/Game/Blueprint/Attribute/AttributeObject.init` _output_get_2))
    (:`then_2`
      (bind _returnvalue_3 (`|GenericCreateObject` "/Game/Blueprint/Attribute/AttributeObject.AttributeObject_C" self))
      (bind _output_get_3 (set `self.buff` _returnvalue_3))
      (`/Game/Blueprint/Attribute/AttributeObject.init` _output_get_3))))

(fn `remove`
  (params (buff :type "/Game/Blueprint/Attribute/AttributeBuff Object Reference"))
  (returns (succ :type Boolean))
  ;[1 1 1] 移除BUFF
  (bind _returnvalue (`KismetArrayLibrary.Array_RemoveItem` (`self.buff_list`) buff))
  (return _returnvalue))