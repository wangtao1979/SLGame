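; AttributeBuff is a turn-based attribute buff, tagged with a module, that holds a Buff and a BuffPer attribute object (apparently flat and percentage bonuses).
; Start derives the end turn from the kept duration, which Init zeroes and SetKeepTurn sets.
; IsActive passes until that turn or always for permanent buffs, and End sets it to -1.
; Count adds both objects, when valid, into the caller's accumulators without checking activity.
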(fn `count`
  (params (input_buff :type "/Game/Blueprint/Attribute/AttributeObject Object Reference") (input_buff_per :type "/Game/Blueprint/Attribute/AttributeObject Object Reference"))
  (returns (buff :type "/Game/Blueprint/Attribute/AttributeObject Object Reference") (buff_per :type "/Game/Blueprint/Attribute/AttributeObject Object Reference"))
  ;[1 1 1] 统计本的BUFF加成属性
  (bind _buff (`self.buff`)
    (:`then`
      (`/Game/Blueprint/Attribute/AttributeObject.add` input_buff _buff))
    (:`else`
      _))
  (bind _buff_per (`self.buff_per`)
    (:`then`
      (`/Game/Blueprint/Attribute/AttributeObject.add` input_buff_per _buff_per))
    (:`else`
      _))
  (return input_buff input_buff_per))

(fn `end`
  ;[1 1 1] 结束BUFF
  (set `self.end_turn` -1))

(fn `get_buff_object`
  (returns (buff_per :type "/Game/Blueprint/Attribute/AttributeObject Object Reference"))
  (return (`self.buff`)))

(fn `get_buff_per_object`
  (returns (buff :type "/Game/Blueprint/Attribute/AttributeObject Object Reference"))
  (return (`self.buff_per`)))

(fn `get_moudle`
  (returns (moudle :type "/Game/Blueprint/Attribute/AttributeBuffTypeEnum Enum"))
  (return (`self.moudle`)))

(fn `init`
  (params (moudle :type "/Game/Blueprint/Attribute/AttributeBuffTypeEnum Enum") (always_exist :type Boolean) (keep_turn :type Integer) (buff :type "/Game/Blueprint/Attribute/AttributeObject Object Reference") (buff_per :type "/Game/Blueprint/Attribute/AttributeObject Object Reference"))
  (set `self.moudle` moudle)
  (set `self.always_exist` always_exist)
  (set `self.keep_turn` 0)
  (set `self.buff` buff)
  (set `self.buff_per` buff_per))

(fn `is_active`
  (params (turn :type Integer))
  (returns (is_active :type Boolean))
  ;[1 1 1] 判断BUFF是否存活
  (return (or (<= turn (`self.end_turn`)) (`self.always_exist`))))

(fn `set_keep_turn`
  (params (keep_turn :type Integer))
  (set `self.keep_turn` keep_turn))

(fn `start`
  (params (turn :type Integer))
  ;[1 1 1] 开始一个BUFF
  (bind _output_get (set `self.begine_turn` turn))
  (set `self.end_turn` (+ _output_get (`self.keep_turn`))))