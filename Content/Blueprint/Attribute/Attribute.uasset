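; Attribute manages a unit's stats, health, action points (AP) and shield.
; Init builds one buff container per module enum entry; adding or removing a buff triggers Compute.
; Compute sums module containers, applies the last as a global modifier, then caps HP and refills AP, keeping previous totals for CountChange notifications.
; SubHp drains shield before HP and fires absorb, damage and death events; CloneState copies state from another Attribute.
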(event `self.ReceiveBeginPlay`
  (`self.init`)
  (`self.InitComplete`))

(event `self.ReceiveEndPlay`
  (params (EndPlayReason :type "EEndPlayReason Enum" :default "Destroyed"))
  (set `self.hp` 0.0)
  (set `self.ap` 0))

(fn `add_attribute_buff`
  (params (buff :type "/Game/Blueprint/Attribute/AttributeBuff Object Reference"))
  (`/Game/Blueprint/Attribute/AttributeBuffContainer.add` (`KismetArrayLibrary.Array_Get` (`self.buff_container_list`) (`KismetMathLibrary.Conv_ByteToInt` (`/Game/Blueprint/Attribute/AttributeBuff.get_moudle` buff))) buff)
  (`self.compute`))

(fn `add_hp`
  (params (hp :type "Float (double-precision)"))
  (bind _hp (`self.hp`))
  (bind _returnvalue (+ _hp hp))
  (if (and (< _hp 0.0) (> _returnvalue 0.0))
    (`self.Revive`))
  (set `self.hp` (`KismetMathLibrary.FMin` _returnvalue (`/Game/Blueprint/Attribute/AttributeObject.get` (`self.final_data`) "NewEnumerator1"))))

(fn `buff_complete`)

(fn `clear`
  (`/Game/Blueprint/Attribute/AttributeObject.clear` (`self.final_data`))
  (`/Game/Blueprint/Attribute/AttributeObject.clear` (`self.last_final_data`))
  (for _array_element (`self.buff_container_list`)
    (`/Game/Blueprint/Attribute/AttributeBuffContainer.clear` _array_element)))

(fn `clear_ap`
  (set `self.ap` 0))

(fn `clone_state`
  (params (attribute :type "/Game/Blueprint/Attribute/Attribute Object Reference"))
  (set `self.hp` (* (`self.get_max_hp`) (* (`self.get_hp_scale` attribute) (`self.hp`))))
  (set `self.ap` (`KismetMathLibrary.Max` (- (`self.get_max_ap`) (`self.get_expend_ap` attribute))))
  (set `self.buff_container_list` (`/Game/Blueprint/Attribute/Attribute.buff_container_list` attribute))
  (`self.compute`))

(fn `compute`
  (bind _buff_container_list (`self.buff_container_list`))
  (bind _final_data (`self.final_data`))
  ;[1 1 1] 计算整个属性
  (`/Game/Blueprint/Attribute/AttributeObject.copy` (`self.last_final_data`) _final_data)
  (`/Game/Blueprint/Attribute/AttributeObject.clear` _final_data)
  (for (_array_element _array_index) _buff_container_list
    (if (!= _array_index (`KismetArrayLibrary.Array_LastIndex` _buff_container_list))
      ;[1 1 1] 模块属性加成
      (bind _attribute (`/Game/Blueprint/Attribute/AttributeBuffContainer.compute` _array_element null))
      (`/Game/Blueprint/Attribute/AttributeObject.add` (`self.final_data`) _attribute)
      (else
        ;[1 1 1] 全局属性加成
        (bind _attribute_2 (`/Game/Blueprint/Attribute/AttributeBuffContainer.compute` _array_element (`self.final_data`)))
        (`/Game/Blueprint/Attribute/AttributeObject.copy` (`self.final_data`) _attribute_2)
        ;[1 1 1] Comment
        (set `self.hp` (`KismetMathLibrary.FMin` (`self.hp`) (`self.get_max_hp`)))
        (set `self.ap` (`self.get_max_ap`))))))

(fn `count_change`
  ;[1 1 1] 统计属性是增加还是减少了
  (for (_array_element _array_index) (`/Game/Blueprint/Attribute/AttributeObject.get_all` (`self.last_final_data`))
    (bind _item (`KismetArrayLibrary.Array_Get` (`/Game/Blueprint/Attribute/AttributeObject.get_all` (`self.final_data`)) _array_index))
    (bind _returnvalue (- _array_element _item))
    (if (!= _returnvalue 0.0)
      (if (< _returnvalue 0.0)
        (bind _define (`self.index_to_define` _array_index))
        (`self.reduceNotify` _define _array_element _item)
        (elif (> _returnvalue 0.0)
          (`self.IncreaseNotify` _define _array_element _item))))))

(fn `define_to_index`
  (params (define :type "/Game/Blueprint/Attribute/AttributeDefine Enum"))
  (returns (index :type Integer))
  ;[1 1 1] 从属性定义转到索引
  (return (`KismetMathLibrary.Conv_ByteToInt` define)))

(fn `force_dead`
  (set `self.hp` 0.0))

(fn `force_revive`
  (set `self.hp` (`self.get_speed`)))

(fn `get_ap`
  (returns (ap :type Integer))
  (return (`self.ap`)))

(fn `get_attribute`
  (params (define :type "/Game/Blueprint/Attribute/AttributeDefine Enum"))
  (returns (value :type "Float (double-precision)"))
  (return (`/Game/Blueprint/Attribute/AttributeObject.get` (`self.final_data`) define)))

(fn `get_dync_attribute`
  (params (define :type "/Game/Blueprint/Attribute/AttributeDefine Enum"))
  (returns (value :type "Float (double-precision)"))
  (if (`|EnumEquality` define "NewEnumerator1")
    (return (`self.get_hp`))
    (else
      (return 0.0))))

(fn `get_expend_ap`
  (returns (ap :type Integer))
  (return (- (`self.get_max_ap`) (`self.get_ap`))))

(fn `get_expend_hp`
  (returns (hp :type "Float (double-precision)"))
  (return (- (`self.get_max_hp`) (`self.hp`))))

(fn `get_hp`
  (returns (hp :type "Float (double-precision)"))
  ;[1 1 1] 获取当前生命
  (return (`self.hp`)))

(fn `get_hp_scale`
  (returns (scale :type "Float (double-precision)"))
  (return (/ (`self.hp`) (`self.get_max_hp`))))

(fn `get_max_ap`
  (returns (ap :type Integer))
  (return (`KismetMathLibrary.FTrunc` (`self.get_attribute` "NewEnumerator4"))))

(fn `get_max_hp`
  (returns (max_hp :type "Float (double-precision)"))
  (return (`/Game/Blueprint/Attribute/AttributeObject.get` (`self.final_data`) "NewEnumerator1")))

(fn `get_orign_attribute`
  (params (define :type "/Game/Blueprint/Attribute/AttributeDefine Enum"))
  (returns (value :type "Float (double-precision)"))
  (return (`/Game/Blueprint/Attribute/AttributeObject.get` (`/Game/Blueprint/Attribute/AttributeBuffContainer.get_attribute` (`KismetArrayLibrary.Array_Get` (`self.buff_container_list`))) define)))

(fn `get_shild_hp`
  (returns (shild_hp :type "Float (double-precision)"))
  (return (`self.shild_hp`)))

(fn `get_shild_hp_scale`
  (returns (shild_hp :type "Float (double-precision)"))
  (return (/ (`self.shild_hp`) (`self.max_shild_hp`))))

(fn `get_speed`
  (returns (speed :type "Float (double-precision)"))
  ;[1 1 1] 获取当前速度
  (return (`/Game/Blueprint/Attribute/AttributeObject.get` (`self.final_data`) "NewEnumerator8")))

(fn `index_to_define`
  (params (index :type Integer))
  (returns (define :type "/Game/Blueprint/Attribute/AttributeDefine Enum"))
  ;[1 1 1] 从索引转到属性枚举
  (return (cast `/Game/Blueprint/Attribute/AttributeDefine` (`KismetMathLibrary.Conv_IntToByte` index))))

(fn `init`
  ;[1 1 1] 初始化属性
  (if (not (`self.is_initial`))
    (`|ExecutionSequence`
      (:`then_0`
        (bind _returnvalue (`|GenericCreateObject` "/Game/Blueprint/Attribute/AttributeObject.AttributeObject_C" self))
        (`/Game/Blueprint/Attribute/AttributeObject.init` _returnvalue)
        (set `self.final_data` _returnvalue))
      (:`then_1`
        (for _ (range (enumcount `/Game/Blueprint/Attribute/AttributeBuffTypeEnum`))
          (bind _returnvalue_2 (`|GenericCreateObject` "/Game/Blueprint/Attribute/AttributeBuffContainer.AttributeBuffContainer_C" self))
          (`/Game/Blueprint/Attribute/AttributeBuffContainer.init` _returnvalue_2)
          (`KismetArrayLibrary.Array_Add` (`self.buff_container_list`) _returnvalue_2)))
      (:`then_2`
        (bind _returnvalue_3 (`|GenericCreateObject` "/Game/Blueprint/Attribute/AttributeObject.AttributeObject_C" self))
        (`/Game/Blueprint/Attribute/AttributeObject.init` _returnvalue_3)
        (set `self.last_final_data` _returnvalue_3))
      (:`then_3`
        (set `self.is_initial` true)))))

(fn `init_complete`
  (`self.compute`)
  (`self.reset_hp`)
  (`self.reset_ap`))

(fn `is_alive`
  (returns (alive :type Boolean))
  (return (> (`self.hp`) 0.0)))

(fn `is_full_ap`
  (returns (is_full :type Boolean))
  (return (== (`self.ap`) (`self.get_max_ap`))))

(fn `remove_attribute_buff`
  (params (buff :type "/Game/Blueprint/Attribute/AttributeBuff Object Reference"))
  (`/Game/Blueprint/Attribute/AttributeBuffContainer.remove` (`KismetArrayLibrary.Array_Get` (`self.buff_container_list`) (`KismetMathLibrary.Conv_ByteToInt` (`/Game/Blueprint/Attribute/AttributeBuff.get_moudle` buff))) buff)
  (`self.compute`))

(fn `reset_ap`
  ;[1 1 1] 重置active point
  (set `self.ap` (`KismetMathLibrary.FTrunc` (`/Game/Blueprint/Attribute/AttributeObject.get` (`self.final_data`) "NewEnumerator4"))))

(fn `reset_hp`
  ;[1 1 1] 重置active point
  (set `self.hp` (`/Game/Blueprint/Attribute/AttributeObject.get` (`self.final_data`) "NewEnumerator1")))

(fn `set_hp_scale`
  (params (scale :type "Float (double-precision)"))
  (set `self.hp` (* (`self.get_max_hp`) scale)))

(fn `set_shild_hp`
  (params (shield :type "Float (double-precision)"))
  (set `self.shild_hp` shield)
  (set `self.max_shild_hp` shield))

(fn `sub_ap`
  (params (ap :type Integer))
  (returns (succ :type Boolean))
  (bind _ap (`self.ap`))
  ;[1 1 1] 消耗AP
  (if (>= _ap ap)
    (set `self.ap` (- _ap ap))
    (return true)
    (else
      (return false))))

(fn `sub_hp`
  (params (sub :type "Float (double-precision)"))
  (returns (hp :type "Float (double-precision)"))
  (locals (sub_hp_value :type "Float (double-precision)") (absorbs_damage :type "Float (double-precision)" :default 0.0))
  (set `local.sub_hp_value` sub)
  (if (> (`self.shild_hp`) 0.0)
    (bind _output_get (set `local.absorbs_damage` (`KismetMathLibrary.FMin` (`local.sub_hp_value`) (`self.shild_hp`))))
    (`self.OnAbsorbsDamage` _output_get)
    (set `self.shild_hp` (- (`self.shild_hp`) (`local.absorbs_damage`)))
    (set `local.sub_hp_value` (- (`local.sub_hp_value`) (`local.absorbs_damage`))))
  (bind _output_get_2 (set `self.hp` (- (`self.hp`) (`local.sub_hp_value`))))
  (if (not (> _output_get_2 0.0))
    (set `self.hp` 0.0)
    (`self.Dead`))
  (`self.OnDamage` (`local.sub_hp_value`))
  (return (`self.hp`)))