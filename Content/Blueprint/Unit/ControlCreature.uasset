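; ControlCreature is a Blueprint for a controllable creature unit that exposes touch, drag and selection controls.
; Small functions toggle the drag flag, the SelectMark's visibility and the capsule's collision, and a getter returns its pass-block type.
; Tap input forwards to CallTap and returns false.
; EnableCollision and DisableCollision set the capsule opposite to their names, mirroring DisableTouch and EnableTouch respectively.
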(event `self.ReceiveBeginPlay`
  (`parent.ReceiveBeginPlay`))

(fn `disable_collision`
  (`PrimitiveComponent.SetCollisionEnabled` (`self.CapsuleComponent`) "QueryAndPhysics"))

(fn `disable_drag`
  (set `self.is_dragdrop` false))

(fn `disable_select`
  (`SceneComponent.SetVisibility` (`self.SelectMark`) false false))

(fn `disable_touch`
  (`PrimitiveComponent.SetCollisionEnabled` (`self.CapsuleComponent`) "NoCollision"))

(fn `enable_collision`
  (`PrimitiveComponent.SetCollisionEnabled` (`self.CapsuleComponent`) "NoCollision"))

(fn `enable_drag`
  (set `self.is_dragdrop` true))

(fn `enable_select`
  (`SceneComponent.SetVisibility` (`self.SelectMark`) true false))

(fn `enable_touch`
  (`PrimitiveComponent.SetCollisionEnabled` (`self.CapsuleComponent`) "QueryAndPhysics"))

(fn `get_pass_type`
  (returns (pass_block_type :type "/Game/Game/Blueprints/WarChess/Scene/Data/TileTypeEnum Enum"))
  (return (`self.pass_block_type`)))

(fn `OnInputTap`
  (returns (ReturnValue :type Boolean))
  (`self.Tap`)
  (return false))

(fn `UserConstructionScript`
  (`parent.UserConstructionScript`))