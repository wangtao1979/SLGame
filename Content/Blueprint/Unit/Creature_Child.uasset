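; Creature_Child is a creature unit Blueprint that carries stub handlers for touch-style input and selection.
; Every tap, hold, swipe and selection function, along with NeedDealSwipe, returns false without doing any work.
; The construction script only calls its parent, and BeginPlay is a disabled placeholder, so the graphs add no behavior of their own.
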(fn `NeedDealSwipe`
  (returns (ReturnValue :type Boolean))
  (return false))

(fn `OnInputHold`
  (returns (ReturnValue :type Boolean))
  (return false))

(fn `OnInputHoldReleased`
  (params (DownTime :type "Float (double-precision)"))
  (returns (ReturnValue :type Boolean))
  (return false))

(fn `OnInputSwipeReleased`
  (params (DeltaPosition :type "Vector Structure (by ref)") (DownTime :type "Float (double-precision)"))
  (returns (ReturnValue :type Boolean))
  (return false))

(fn `OnInputSwipeStart`
  (params (StartPosition :type "Vector Structure (by ref)"))
  (returns (ReturnValue :type Boolean))
  (return false))

(fn `OnInputSwipeUpdate`
  (params (DeltaPosition :type "Vector Structure (by ref)"))
  (returns (ReturnValue :type Boolean))
  (return false))

(fn `OnInputTap`
  (returns (ReturnValue :type Boolean))
  (return false))

(fn `OnSelectionGained`
  (params (InputType :type "ETouchInputEnum Enum" :default "VE_Tap"))
  (returns (ReturnValue :type Boolean))
  (return false))

(fn `OnSelectionLost`
  (params (NewPosition :type "Vector Structure (by ref)") (NewActor :type "Actor Object Reference") (InputType :type "ETouchInputEnum Enum" :default "VE_Tap"))
  (returns (ReturnValue :type Boolean))
  (return false))

(fn `UserConstructionScript`
  (`parent.UserConstructionScript`))