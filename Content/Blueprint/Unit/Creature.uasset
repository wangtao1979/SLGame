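; Base creature unit Blueprint that provides shared visual, transform and socket helpers, caching original materials, textures, mesh scale and play rate on BeginPlay.
; Material overrides use a stack, recursively creating dynamic instances across child meshes that keep each slot's BaseTexture, with restore and parameter setters.
; Other functions handle facing, snapping to actors, scaling, animation speed or freezing, capsule size, and LaunchPoint socket lookup for bullets.
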(event `self.ReceiveBeginPlay`
  (`self.InitMaterial` (`self.Mesh`))
  (`self.InitTransform`)
  (`self.InitAnimation`))

(fn `CreateDynamicMaterial`
  (params (mesh_component :type "MeshComponent Object Reference") (material :type "MaterialInterface Object Reference") (index :type Integer))
  (returns (reslut_index :type Integer))
  (locals (new_material :type "MaterialInterface Object Reference") (cur_mesh :type "MeshComponent Object Reference") (cur_index :type Integer))
  (set `local.cur_mesh` mesh_component)
  (set `local.cur_index` index)
  (set `local.new_material` material)
  (for (_ _array_index) (`MeshComponent.GetMaterials` (`local.cur_mesh`))
    (bind _returnvalue (+ _array_index (`local.cur_index`)))
    (bind _returnvalue_2 (`PrimitiveComponent.CreateDynamicMaterialInstance` (`local.cur_mesh`) _array_index (select `bool` (`KismetSystemLibrary.IsValid` (`local.new_material`)) :`false` (`KismetArrayLibrary.Array_Get` (`self.BaseMaterial`) _returnvalue) :`true` (`local.new_material`))))
    (`MaterialInstanceDynamic.SetTextureParameterValue` _returnvalue_2 "BaseTexture" (`KismetArrayLibrary.Array_Get` (`self.BaseTexture`) _returnvalue))
    (`KismetArrayLibrary.Array_Add` (`self.DynamicMaterial`) _returnvalue_2))
  (set `local.cur_index` (+ (`local.cur_index`) (`PrimitiveComponent.GetNumMaterials` (`local.cur_mesh`))))
  (for _array_element (`SceneComponent.GetChildrenComponents` (`local.cur_mesh`) false)
    (bind _asmesh_component (cast `MeshComponent` _array_element))
    (bind _reslut_index (`self.CreateDynamicMaterial` _asmesh_component (`local.new_material`) (`local.cur_index`)))
    (set `local.cur_index` _reslut_index))
  (return (`local.cur_index`)))

(fn `GetBulletLauchTransform`
  (returns (transform :type "Transform Structure"))
  (for _array_element (`SceneComponent.GetChildrenComponents` (`self.Mesh`) false)
    (bind _asmesh_component (cast `MeshComponent` _array_element))
    (for _array_element_2 (`SceneComponent.GetAllSocketNames` _asmesh_component)
      (if (== _array_element_2 "LaunchPoint")
        (return (`SceneComponent.GetSocketTransform` _asmesh_component "LaunchPoint" "RTS_World")))))
  (return (`SceneComponent.GetSocketTransform` (`self.Mesh`) "LaunchPoint" "RTS_World")))

(fn `GetCapsuleHalfHeight`
  (returns (half_height :type "Float (double-precision)"))
  (return (`CapsuleComponent.GetScaledCapsuleHalfHeight` (`self.CapsuleComponent`))))

(fn `GetCapsuleRadius`
  (returns (radius :type "Float (double-precision)"))
  (return (`CapsuleComponent.GetScaledCapsuleRadius` (`self.CapsuleComponent`))))

(fn `InitAnimation`
  (bind _output_get (set `self.OriginalSpeed` (`SkeletalMeshComponent.GetPlayRate` (`self.Mesh`))))
  (set `self.AnimationSpeed` _output_get))

(fn `InitMaterial`
  (params (mesh_component :type "MeshComponent Object Reference"))
  (for _array_element (`MeshComponent.GetMaterials` mesh_component)
    (`KismetArrayLibrary.Array_Add` (`self.BaseMaterial`) _array_element)
    (bind _returnvalue (`MaterialFunctionLibrary.GetParameterTexture` _array_element "BaseTexture"))
    (`KismetArrayLibrary.Array_Add` (`self.BaseTexture`) _returnvalue))
  (for _array_element_2 (`SceneComponent.GetChildrenComponents` mesh_component false)
    (bind _asmesh_component (cast `MeshComponent` _array_element_2))
    (`self.InitMaterial` _asmesh_component)))

(fn `InitTransform`
  (set `self.OriginalMeshScale` (`SceneComponent.K2_GetComponentScale` (`self.Mesh`))))

(fn `LocationToActor`
  (params (actor :type "Actor Object Reference") (rotation_actor :type "Actor Object Reference"))
  (bind (_returnvalue_x _returnvalue_y) (`KismetMathLibrary.BreakVector` (`self.K2_GetActorLocation` actor)))
  (bind _returnvalue (`self.GetTransform`))
  (`self.K2_SetActorTransform` (`KismetMathLibrary.MakeTransform` (`KismetMathLibrary.MakeVector` _returnvalue_x _returnvalue_y (.z (.location _returnvalue))) (`self.K2_GetActorRotation` rotation_actor) (.scale _returnvalue)) false true))

(fn `Lookat`
  (params (actor :type "Actor Object Reference"))
  (bind (_returnvalue_x _returnvalue_y) (`KismetMathLibrary.BreakVector` (`self.K2_GetActorLocation` actor)))
  (bind (_returnvalue_x_2 _returnvalue_y_2) (`KismetMathLibrary.BreakVector` (`self.K2_GetActorLocation`)))
  (if (`KismetSystemLibrary.IsValid` actor)
    (`self.K2_SetActorRotation` (`KismetMathLibrary.FindLookAtRotation` (`KismetMathLibrary.MakeVector` _returnvalue_x_2 _returnvalue_y_2) (`KismetMathLibrary.MakeVector` _returnvalue_x _returnvalue_y)))))

(fn `RestorMaterial`
  (`KismetArrayLibrary.Array_Clear` (`self.DynamicMaterial`))
  (if (> (`KismetArrayLibrary.Array_Length` (`self.MaterialStack`)) 1)
    (`KismetArrayLibrary.Array_Remove` (`self.MaterialStack`) (`KismetArrayLibrary.Array_LastIndex` (`self.MaterialStack`)))
    (`self.CreateDynamicMaterial` (`self.Mesh`) (`KismetArrayLibrary.Array_Get` (`self.MaterialStack`) (`KismetArrayLibrary.Array_LastIndex` (`self.MaterialStack`))))
    (else
      (`KismetArrayLibrary.Array_Clear` (`self.MaterialStack`))
      (`self.CreateDynamicMaterial` (`self.Mesh`)))))

(fn `RotateAsActor`
  (params (actor :type "Actor Object Reference"))
  (`self.K2_SetActorRotation` (`self.K2_GetActorRotation` actor)))

(fn `Scale`
  (params (scale :type "Float (double-precision)"))
  (`self.SetActorScale3D` (* (`self.OriginalMeshScale`) scale)))

(fn `SetAnimationSpeed`
  (params (speed :type "Float (double-precision)"))
  (set `self.AnimationSpeed` (* speed (`self.OriginalSpeed`))))

(fn `SetDynamicColor`
  (params (name :type Name) (color :type "LinearColor Structure"))
  (for _array_element (`self.DynamicMaterial`)
    (`MaterialInstanceDynamic.SetVectorParameterValue` _array_element name color)))

(fn `SetDynamicTexture`
  (params (name :type Name) (texture :type "Texture Object Reference"))
  (for _array_element (`self.DynamicMaterial`)
    (`MaterialInstanceDynamic.SetTextureParameterValue` _array_element name texture)))

(fn `SetDynamicValue`
  (params (name :type Name) (value :type "Float (double-precision)"))
  (for _array_element (`self.DynamicMaterial`)
    (`MaterialInstanceDynamic.SetScalarParameterValue` _array_element name value)))

(fn `SetMaterial`
  (params (new_materal :type "MaterialInterface Object Reference"))
  (`/Engine/EditorBlueprintResources/StandardMacros.IsValid` new_materal
    (:`Is Valid`
      (`KismetArrayLibrary.Array_Add` (`self.MaterialStack`) new_materal)
      (`KismetArrayLibrary.Array_Clear` (`self.DynamicMaterial`))
      (`self.CreateDynamicMaterial` (`self.Mesh`) new_materal))))

(fn `StopAnimation`
  (bind _mesh (`self.Mesh`)
    (:`then`
      (set `SkeletalMeshComponent.GlobalAnimRateScale` 0.0 _mesh))
    (:`else`)))

(fn `UserConstructionScript`)