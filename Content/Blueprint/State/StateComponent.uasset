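; StateComponent is a component that tracks which states are active on its owner, as driven by buffs.
; On BeginPlay it constructs one StateContainer per enum entry, so the enum value serves directly as the index into StateList.
; AddBuff and RemoveBuff register or unregister a state object in the container of every state that its GetState returns.
; IsStateActive delegates the query to the container at the requested state's index.
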(event `self.ReceiveBeginPlay`
  (for _ (range (+ (enumcount `/Game/Blueprint/State/CreatureStateEnum`) 1))
    (bind _returnvalue (`|GenericCreateObject` "/Game/Blueprint/State/StateContainer.StateContainer_C" self))
    (`KismetArrayLibrary.Array_Add` (`self.state_list`) _returnvalue)))

(fn `add_buff`
  (params (state :type "/Game/Blueprint/State/ICreatureState Interface"))
  (bind _state_list (`/Game/Blueprint/State/ICreatureState.GetState` state))
  (for _array_element _state_list
    (`/Game/Blueprint/State/StateContainer.add` (`KismetArrayLibrary.Array_Get` (`self.state_list`) (`KismetMathLibrary.Conv_ByteToInt` _array_element)) state)))

(fn `is_state_active`
  (params (state :type "/Game/Blueprint/State/CreatureStateEnum Enum"))
  (returns (active :type Boolean))
  (return (`/Game/Blueprint/State/StateContainer.is_active` (`KismetArrayLibrary.Array_Get` (`self.state_list`) (`KismetMathLibrary.Conv_ByteToInt` state)))))

(fn `remove_buff`
  (params (state :type "/Game/Blueprint/State/ICreatureState Interface"))
  (bind _state_list (`/Game/Blueprint/State/ICreatureState.GetState` state))
  (for _array_element _state_list
    (`/Game/Blueprint/State/StateContainer.remove` (`KismetArrayLibrary.Array_Get` (`self.state_list`) (`KismetMathLibrary.Conv_ByteToInt` _array_element)) state)))