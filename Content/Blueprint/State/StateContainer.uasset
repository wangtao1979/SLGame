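; StateContainer holds a list of state buffs and reports whether any of them is active.
; Add inserts a state without duplicates, Remove drops one, and Clear empties the list.
; IsActive loops over the list and returns true at the first entry whose own IsActive is true, otherwise false.
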(fn `add`
  (params (state :type "/Game/Blueprint/State/ICreatureState Interface"))
  (`KismetArrayLibrary.Array_AddUnique` (`self.state_buff_list`) state))

(fn `clear`
  (`KismetArrayLibrary.Array_Clear` (`self.state_buff_list`)))

(fn `is_active`
  (returns (active :type Boolean))
  (for _array_element (`self.state_buff_list`)
    (bind _active (`/Game/Blueprint/State/ICreatureState.IsActive` _array_element))
    (if _active
      (return true)))
  (return false))

(fn `remove`
  (params (buff :type "/Game/Blueprint/State/ICreatureState Interface"))
  (`KismetArrayLibrary.Array_RemoveItem` (`self.state_buff_list`) buff))