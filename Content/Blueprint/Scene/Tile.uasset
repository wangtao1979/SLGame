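; Tile actor for a six-neighbour, turn-based tactics map that holds creatures, answers pass and stand checks, and forwards taps to the controlled creature.
; A state enum recolours a dynamic material for move and spell-targeting highlights.
; Pathfinding, distance and range queries run HeroLevel's BFS with lazily created hook objects, while line and rotatable mask-tree queries step through grid coordinates.
; It also serializes edges and creatures and caches per-direction AI scores.
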(event `self.ReceiveBeginPlay`
  (`self.HeroLevel`
    (:`then`)
    (:`else`
      (bind _outactors (`GameplayStatics.GetAllActorsOfClass` "/Game/Blueprint/Scene/HeroLevel.HeroLevel_C"))
      (set `self.HeroLevel` (`KismetArrayLibrary.Array_Get` _outactors)))))

(event `SetGuid`
  ;[1 1 1] 设置引导信息
  (`|SpawnActorFromClass` null (`self.GetTransform`) "AlwaysSpawn" "OverrideRootScale")
  (set `self.Guider` null)
  (`self.SetCondtion` (struct)))

(event `self.ReceiveEndPlay`
  (params (EndPlayReason :type "EEndPlayReason Enum" :default "Destroyed"))
  (`self.Guider`
    (:`then`
      (`self.K2_DestroyActor`))
    (:`else`)))

(fn `add_creature`
  (params (creature :type "Object Object Reference"))
  (`KismetArrayLibrary.Array_AddUnique` :`NewItem` creature))

(fn `can_pass`
  (params (creature :type "Object Object Reference"))
  (returns (cann_pass :type Boolean))
  (locals (tile_creature :type "Object Object Reference"))
  (return (or (>= (`self.get_pass_type` creature) (`self.get_pass_type_with_creature`)) (== (`self.get_tile` creature) self))))

(fn `can_stand`
  (params (crature :type "Object Object Reference"))
  (returns (can_stand :type Boolean))
  (return (or (== (`self.get_tile` crature) self) (<= (`self.get_pass_type_with_creature`) (enumliteral `/Game/Game/Blueprints/WarChess/Scene/Data/TileTypeEnum` "NewEnumerator0")))))

(fn `check_physice_passable`
  (params (target :type "/Game/Blueprint/Scene/Tile Object Reference"))
  (returns (can_pass :type Boolean))
  (bind _path (`self.get_distance` target))
  (for _index (range 1 (+ (`KismetArrayLibrary.Array_LastIndex` _path) 1))
    (if (not false)
      (return false)))
  (return true))

(fn `control_creature_can_pass`
  (returns (CanPass :type Boolean))
  (return (`self.can_pass` null)))

(fn `control_creature_can_stand`
  (returns (CanPass :type Boolean))
  (return (`self.can_stand` null)))

(fn `disable_guid`
  (`self.Guider`
    (:`then`
      (`self.Disable`))
    (:`else`)))

(fn `ExtendGetDir`
  (params (dest_tile :type "/Game/Blueprint/Scene/Tile Object Reference"))
  (returns (dir :type Integer))
  (if (!= dest_tile self)
    (bind _path (`self.FindPath` dest_tile false))
    (bind _dir (`self.GetDir` (`KismetArrayLibrary.Array_Get` _path (- (`KismetArrayLibrary.Array_LastIndex` _path) 1))))
    (return _dir)
    (else
      (return 0))))

(fn `FindPath`
  (params (DstTile :type "/Game/Blueprint/Scene/Tile Object Reference") (block :type Boolean :default false) (step :type Integer :default 16))
  (returns (Path :type "Array of /Game/Blueprint/Scene/Tile Object Reference"))
  (`|ExecutionSequence`
    (:`then_0`
      (`self.FindPathHooker`
        (:`then`)
        (:`else`
          (bind _returnvalue (`|GenericCreateObject` "/Game/Game/Blueprints/WarChess/Scene/Logic/BFSHookFindPath.BFSHookFindPath_C" self))
          (set `self.FindPathHooker` _returnvalue))))
    (:`then_1`
      (set `/Game/Game/Blueprints/WarChess/Scene/Logic/BFSHookFindPath.DstTarget` self (`self.FindPathHooker`))
      (`/Game/Blueprint/Scene/HeroLevel.Bfs` (`self.get_map`) step block DstTile (`self.FindPathHooker`))
      (return (`/Game/Game/Blueprints/WarChess/Scene/Logic/BFSHookFindPath.Path` (`self.FindPathHooker`))))))

(fn `get_creature`
  (returns (creatue :type "Object Object Reference"))
  (if (<= (`KismetArrayLibrary.Array_Length` _) 0)
    (return null)
    (else
      (return (`KismetArrayLibrary.Array_Get` :`Index` (`KismetArrayLibrary.Array_LastIndex` _))))))

(fn `get_distance`
  (params (dest :type "/Game/Blueprint/Scene/Tile Object Reference"))
  (returns (Path :type "Array of /Game/Blueprint/Scene/Tile Object Reference"))
  (`|ExecutionSequence`
    (:`then_0`
      (`self.DistanceHooker`
        (:`then`)
        (:`else`
          (bind _returnvalue (`|GenericCreateObject` "/Game/Game/Blueprints/WarChess/Scene/Logic/BFSHookDistance.BFSHookDistance_C" self))
          (set `self.DistanceHooker` _returnvalue))))
    (:`then_1`
      (set `/Game/Game/Blueprints/WarChess/Scene/Logic/BFSHookDistance.DstTarget` dest (`self.DistanceHooker`))
      (`/Game/Blueprint/Scene/HeroLevel.Bfs` (`self.get_map`) 16 false self (`self.DistanceHooker`))
      (return (`/Game/Game/Blueprints/WarChess/Scene/Logic/BFSHookDistance.Path` (`self.DistanceHooker`))))))

(fn `get_hit_component`
  (returns (component :type "MeshComponent Object Reference"))
  (return (`self.StaticMesh`)))

(fn `get_map`
  (returns (herolevel :type "/Game/Blueprint/Scene/HeroLevel Object Reference"))
  (return (`self.HeroLevel`)))

(fn `get_pass_type_with_creature`
  (returns (type :type "/Game/Game/Blueprints/WarChess/Scene/Data/TileTypeEnum Enum"))
  (locals (tile_creature :type "Object Object Reference"))
  (set `local.tile_creature` null)
  (if (`KismetSystemLibrary.IsValid` null)
    (if (`self.is_alive`)
      (return "NewEnumerator1")
      (else
        _)))
  (return (`self.get_type`)))

(fn `get_tile_index`
  (returns (IndexInMap :type Integer))
  (return (`self.IndexInMap`)))

(fn `get_type`
  (returns (type :type "/Game/Game/Blueprints/WarChess/Scene/Data/TileTypeEnum Enum"))
  (bind _serializationdata_path_type (break `/Game/Game/Blueprints/WarChess/Scene/Data/TileData` (`self.SerializationData`)))
  (return _serializationdata_path_type))

(fn `GetAiCacheScore`
  (params (dir :type Integer))
  (returns (Score :type "Float (double-precision)"))
  (locals (LocalSimple :type Boolean))
  (return (`KismetArrayLibrary.Array_Get` (`self.SimpleScoreList`) dir)))

(fn `GetDir`
  (params (DestTile :type "/Game/Blueprint/Scene/Tile Object Reference"))
  (returns (dir :type Integer))
  (for _index (range 6)
    (bind _item (`KismetArrayLibrary.Array_Get` (`self.Edge`) _index))
    (`/Engine/EditorBlueprintResources/StandardMacros.IsValid` _item
      (:`Is Valid`
        (if (== _item DestTile)
          (return _index)))))
  (return 0))

(fn `GetLineTile`
  (params (Dir :type Integer) (Step :type Integer))
  (returns (Line :type "Array of /Game/Blueprint/Scene/Tile Object Reference"))
  (locals (LocalX :type Integer :default 0) (LocalY :type Integer :default 0) (Result :type "Array of /Game/Blueprint/Scene/Tile Object Reference") (LocalIndex :type Integer))
  (`KismetArrayLibrary.Array_Add` (`local.Result`) self)
  (bind (_x _y) (`/Game/Blueprint/Scene/HeroLevel.IndexToXY` (`self.get_map`) (`self.IndexInMap`)))
  (set `local.LocalX` _x)
  (set `local.LocalY` _y)
  (for _ (range 1 (+ Step 1))
    (bind (_newx _newy) (`/Game/Blueprint/Scene/HeroLevel.MathMoveTo` (`self.get_map`) (`local.LocalX`) (`local.LocalY`) Dir))
    (bind _output_get (set `local.LocalX` _newx))
    (bind _output_get_2 (set `local.LocalY` _newy))
    (bind _index (`/Game/Blueprint/Scene/HeroLevel.XYToIndex` (`self.get_map`) _output_get _output_get_2))
    (bind _output_get_3 (set `local.LocalIndex` _index))
    (if (== -1 _output_get_3)
      (break)
      (else
        (`KismetArrayLibrary.Array_Add` (`local.Result`) (`/Game/Blueprint/Scene/HeroLevel.GetTileByIndex` (`self.get_map`) (`local.LocalIndex`))))))
  (return (`local.Result`)))

(fn `GetMaskTile1`
  (params (Dir :type Integer) (MaskData :type "/Game/Game/Blueprints/WarChess/Scene/Data/MaskData Structure"))
  (returns (TileList :type "Array of /Game/Blueprint/Scene/Tile Object Reference"))
  (locals (ResultTile :type "Array of /Game/Blueprint/Scene/Tile Object Reference") (LocalCreatureDir :type Integer) (LocalTile :type "/Game/Blueprint/Scene/Tile Object Reference") (LocalEdgeDir :type Integer) (GetFirstMaskTile :type Boolean) (LocalMaskSearchNode :type "/Game/Game/Blueprints/WarChess/Scene/Data/MaskSearchNode Structure" :default (struct :`Node` (struct))) (LocalSearchQueue :type "Array of /Game/Game/Blueprints/WarChess/Scene/Data/MaskSearchNode Structure") (LocalX :type Integer :default 0) (LocalY :type Integer) (LocalMaskTileIndex :type Integer) (LocalTree :type "/Game/Game/Blueprints/WarChess/Scene/Data/Tree Structure" :default (struct)))
  (bind _localmasksearchnode (`local.LocalMaskSearchNode`))
  (bind _localtree_allnode (break `/Game/Game/Blueprints/WarChess/Scene/Data/Tree` (`local.LocalTree`)))
  (bind (_localmasksearchnode_node _localmasksearchnode_x _localmasksearchnode_y) (break `/Game/Game/Blueprints/WarChess/Scene/Data/MaskSearchNode` (`local.LocalMaskSearchNode`)))
  (bind _localtree_allnode_2 (break `/Game/Game/Blueprints/WarChess/Scene/Data/Tree` (`local.LocalTree`)))
  (if MaskData_contai_self_10_6183AB2B460AAB30C3D81DB8429EFCA1
    (`KismetArrayLibrary.Array_Add` (`local.ResultTile`) self))
  (set `local.LocalCreatureDir` Dir)
  (for _array_element MaskData_child_mask_8_D9E173CD468BD66C848C49B3C6F32B8A
    (set `local.LocalTree` (break `/Game/Game/Blueprints/WarChess/Scene/Data/ChildMask1` _array_element))
    (bind (_x _y) (`/Game/Blueprint/Scene/HeroLevel.IndexToXY` (`self.HeroLevel`) (`self.IndexInMap`)))
    (set `local.LocalX` _x)
    (set `local.LocalY` _y)
    (for _array_element_2 (`.Path_6_57A83E894DBA68CD6A0F59B5C2AE9758` (break `/Game/Game/Blueprints/WarChess/Scene/Data/ChildMask1` _array_element))
      (bind _output_get (set `local.LocalEdgeDir` (mod (+ _array_element_2 (`local.LocalCreatureDir`)) 6)))
      (bind (_newx _newy) (`/Game/Blueprint/Scene/HeroLevel.MathMoveTo` (`self.HeroLevel`) (`local.LocalX`) (`local.LocalY`) _output_get))
      (set `local.LocalX` _newx)
      (set `local.LocalY` _newy))
    (`KismetArrayLibrary.Array_Add` (`local.LocalSearchQueue`) (make `/Game/Game/Blueprints/WarChess/Scene/Data/MaskSearchNode` (`KismetArrayLibrary.Array_Get` _localtree_allnode) (`local.LocalX`) (`local.LocalY`)))
    (while (> (`KismetArrayLibrary.Array_Length` (`local.LocalSearchQueue`)) 0)
      (set `local.LocalMaskSearchNode` (`KismetArrayLibrary.Array_Get` (`local.LocalSearchQueue`)))
      (`KismetArrayLibrary.Array_Remove` (`local.LocalSearchQueue`))
      (bind _index (`/Game/Blueprint/Scene/HeroLevel.XYToIndex` (`self.HeroLevel`) _localmasksearchnode_x _localmasksearchnode_y))
      (bind _output_get_2 (set `local.LocalMaskTileIndex` _index))
      (if (!= _output_get_2 -1)
        (`KismetArrayLibrary.Array_Add` (`local.ResultTile`) (`/Game/Blueprint/Scene/HeroLevel.GetTileByIndex` (`self.HeroLevel`) (`local.LocalMaskTileIndex`))))
      (for _array_element_3 (break `/Game/Game/Blueprints/WarChess/Scene/Data/TreeNode` (break `/Game/Game/Blueprints/WarChess/Scene/Data/MaskSearchNode` _localmasksearchnode))
        (bind (_newx_2 _newy_2) (`/Game/Blueprint/Scene/HeroLevel.MathMoveTo` (`self.HeroLevel`) (`.X_6_82E5C63B4D135DCB12E2F4B94C9C02F2` (break `/Game/Game/Blueprints/WarChess/Scene/Data/MaskSearchNode` _localmasksearchnode)) (`.Y_7_7BD7BF35448D9B989E600E80FC16CAFE` (break `/Game/Game/Blueprints/WarChess/Scene/Data/MaskSearchNode` _localmasksearchnode)) (mod (+ (`.dir_5_A096A2684C83BAA66E9D4F8A12619CE8` (break `/Game/Game/Blueprints/WarChess/Scene/Data/TreeEdge` _array_element_3)) (`local.LocalCreatureDir`)) 6)))
        (`KismetArrayLibrary.Array_Add` (`local.LocalSearchQueue`) (make `/Game/Game/Blueprints/WarChess/Scene/Data/MaskSearchNode` (`KismetArrayLibrary.Array_Get` _localtree_allnode_2 (break `/Game/Game/Blueprints/WarChess/Scene/Data/TreeEdge` _array_element_3)) _newx_2 _newy_2)))))
  (return (`local.ResultTile`)))

(fn `GetNearTile`
  (params (min_step :type Integer) (max_step :type Integer) (CheckPassable :type Boolean :default false))
  (returns (TileList :type "Array of /Game/Blueprint/Scene/Tile Object Reference"))
  (`|ExecutionSequence`
    (:`then_0`
      (`self.NearListHooker`
        (:`then`)
        (:`else`
          (bind _returnvalue (`|GenericCreateObject` "/Game/Game/Blueprints/WarChess/Scene/Logic/BFSHookNear.BFSHookNear_C" self))
          (set `self.NearListHooker` _returnvalue))))
    (:`then_1`
      (set `/Game/Game/Blueprints/WarChess/Scene/Logic/BFSHookNear.MinStep` min_step (`self.NearListHooker`))
      (`KismetArrayLibrary.Array_Clear` (`/Game/Game/Blueprints/WarChess/Scene/Logic/BFSHookNear.TileList` (`self.NearListHooker`)))
      (bind _output_get (set `/Game/Game/Blueprints/WarChess/Scene/Logic/BFSHookNear.FilterPassable` CheckPassable (`self.NearListHooker`)))
      (`/Game/Blueprint/Scene/HeroLevel.Bfs` (`self.get_map`) max_step _output_get self (`self.NearListHooker`))
      (return (`/Game/Game/Blueprints/WarChess/Scene/Logic/BFSHookNear.TileList` (`self.NearListHooker`))))))

(fn `is_loaction_in_bounds`
  (params (locaiotn :type "Vector Structure"))
  (returns (is_in_bounds :type Boolean))
  (bind _staticmesh (`self.StaticMesh`))
  (bind (_min _max) (`StaticMeshComponent.GetLocalBounds` _staticmesh))
  (bind _returnvalue (`SceneComponent.K2_GetComponentLocation` _staticmesh))
  (bind (_returnvalue_x _returnvalue_y) (`KismetMathLibrary.BreakVector` (+ _returnvalue _min)))
  (bind (_returnvalue_x_2 _returnvalue_y_2) (`KismetMathLibrary.BreakVector` (+ _returnvalue _max)))
  (return (and (> locaiotn_X _returnvalue_x) (< locaiotn_X _returnvalue_x_2) (> locaiotn_Y _returnvalue_y) (< locaiotn_Y _returnvalue_y_2))))

(fn `OnInputTap`
  (returns (ReturnValue :type Boolean))
  (bind _controler (`/Game/Game/Blueprints/WarChess/Fight/turn/TurnManager.get_control_creature` (`self.get_turn_manager`)))
  (`self.Touch` self)
  (`/Engine/EditorBlueprintResources/StandardMacros.IsValid` _controler
    (:`Is Valid`
      (`self.touch_tile` _controler self))
    (:`Is Not Valid`
      (`self.disable_guid`)))
  (return false))

(fn `OnSelectionGained`
  (params (InputType :type Byte :default 0))
  (returns (ReturnValue :type Boolean))
  (return false))

(fn `remove_creature`
  (if (> (`KismetArrayLibrary.Array_Length` _) 0)
    (`KismetArrayLibrary.Array_Remove` :`IndexToRemove` (`KismetArrayLibrary.Array_LastIndex` _))))

(fn `revent_state`
  (`self.set_state` (`self.last_state`)))

(fn `SerializationEdge`
  (params (hero_level :type "/Game/Blueprint/Scene/HeroLevel Object Reference"))
  (bind (_serializationdata_path_type _serializationdata_attach_mesh _serializationdata_edge) (break `/Game/Game/Blueprints/WarChess/Scene/Data/TileData` (`self.SerializationData`)))
  (for (_array_element _array_index) _serializationdata_edge
    (if (!= _array_element -1)
      (`KismetArrayLibrary.Array_Set` (`self.Edge`) _array_index (`/Game/Blueprint/Scene/HeroLevel.GetTileByIndex` hero_level _array_element) true))))

(fn `SerializationFrom`
  (params (TileData :type "/Game/Game/Blueprints/WarChess/Scene/Data/TileData Structure") (hero_level :type "/Game/Blueprint/Scene/HeroLevel Object Reference"))
  (locals (transform :type "Transform Structure"))
  (bind _transform_location (`KismetMathLibrary.BreakTransform` (`local.transform`)))
  (add `/Game/Blueprint/Scene/HeroLevel.SpawnTileEnd` hero_level (`|CreateDelegate` :!event `SerializationEdge`))
  (bind _output_get (set `self.SerializationData` TileData))
  (`SceneComponent.SetVisibility` (`self.DefaultSceneRoot`) (`.visible_34_00238650474B54E050FCB1A3895886C2` (break `/Game/Game/Blueprints/WarChess/Scene/Data/TileData` _output_get)) true)
  (bind _output_get_2 (set `local.transform` (`.transform_22_6D2DC1E34F5249D1D14FC0B391951956` (break `/Game/Game/Blueprints/WarChess/Scene/Data/TileData` _output_get))))
  (`SceneComponent.K2_SetWorldTransform` (`self.DefaultSceneRoot`) _output_get_2 false false)
  (for _array_element (`.creature_26_75A5EA1D46EC3824290416BFF5BC2938` (break `/Game/Game/Blueprints/WarChess/Scene/Data/TileData` _output_get))
    (bind _returnvalue (`|SpawnActorFromClass` null (`KismetMathLibrary.MakeTransform` _transform_location (struct)) "Undefined" "OverrideRootScale"))
    (`self.set_tile` _returnvalue self)
    (`self.SerializationFrom` _returnvalue _array_element))
  (`self.SetGuid`))

(fn `SerializationTo`
  (returns (NewParam :type "/Game/Game/Blueprints/WarChess/Scene/Data/TileData Structure"))
  (bind (_serializationdata_path_type _serializationdata_attach_mesh _serializationdata_edge _serializationdata_transform _serializationdata_creature _serializationdata_visible) (break `/Game/Game/Blueprints/WarChess/Scene/Data/TileData` (`self.SerializationData`)))
  (bind (_serializationdata_path_type_2 _serializationdata_attach_mesh_2 _serializationdata_edge_2 _serializationdata_transform_2 _serializationdata_creature_2) (break `/Game/Game/Blueprints/WarChess/Scene/Data/TileData` (`self.SerializationData`)))
  (bind (_serializationdata_path_type_3 _serializationdata_attach_mesh_3 _serializationdata_edge_3) (break `/Game/Game/Blueprints/WarChess/Scene/Data/TileData` (`self.SerializationData`)))
  (set `self.SerializationData` (make `/Game/Game/Blueprints/WarChess/Scene/Data/TileData` _serializationdata_path_type null _serializationdata_edge (`SceneComponent.K2_GetComponentToWorld` (`self.DefaultSceneRoot`)) _serializationdata_creature _serializationdata_visible))
  (for _array_element (`self.Edge`)
    (`/Engine/EditorBlueprintResources/StandardMacros.IsValid` _array_element
      (:`Is Valid`
        (`KismetArrayLibrary.Array_Add` _serializationdata_edge_3 (`/Game/Blueprint/Scene/Tile.IndexInMap` _array_element)))
      (:`Is Not Valid`
        (`KismetArrayLibrary.Array_Add` _serializationdata_edge_3 -1))))
  (for _array_element_2 _
    ;[1 1 1] 测试导出才会导出玩家角色的数据
    (if (`/Game/Blueprint/Scene/Tile.export_final_data` (`self.get_fight_game_mode`))
      (if (`|EnumInequality` (`self.get_faction` _array_element_2) "NewEnumerator0")
        (bind _data (`self.SerializationTo` _array_element_2 :!label _label))
        (`KismetArrayLibrary.Array_Add` _serializationdata_creature_2 _data))
      (else
        (goto _label))))
  (return (`self.SerializationData`)))

(fn `set_state`
  (params (state :type "/Game/Game/Blueprints/WarChess/Scene/Data/TIleStateEnum Enum"))
  (bind _defaulttiletexture (`self.DefaultTileTexture`))
  (set `self.last_state` (`self.state`))
  (bind _output_get (set `self.state` state))
  (switch `/Game/Game/Blueprints/WarChess/Scene/Data/TIleStateEnum` _output_get
    (:`NewEnumerator4`
      ;[1 1 1] 初始状态
      (`self.set_tile_color` (struct :`R` 0.095 :`G` 0.095 :`B` 0.095) _defaulttiletexture))
    (:`NewEnumerator0`
      ;[1 1 1] 移动范围
      (`self.set_tile_color` (struct :`R` 0.63 :`G` 0.63 :`B` 0.63 :`A` 1.0) _defaulttiletexture))
    (:`NewEnumerator8`
      ;[1 1 1] 敌对法术可选施法范围
      (`self.set_tile_color` (struct :`R` 1.0 :`G` 0.885502 :`A` 1.0) (`self.DefaultTileTexture`)))
    (:`NewEnumerator2`
      ;[1 1 1] 敌对选中目标
      (`self.set_tile_color` (struct :`R` 1.0 :`G` 0.110346 :`A` 1.0) (`self.DefaultTileTexture`)))
    (:`NewEnumerator5`
      ;[1 1 1] 敌方影响范围
      (`self.set_tile_color` (struct :`R` 0.901961 :`G` 0.4 :`A` 1.0) (`self.DefaultTileTexture`)))
    (:`NewEnumerator10`
      ;[1 1 1] 友方法术可选范围
      (`self.set_tile_color` (struct :`R` 1.0 :`G` 0.886275 :`A` 1.0) (`self.DefaultTileTexture`)))
    (:`NewEnumerator6`
      ;[1 1 1] 友方法术选择目标
      (`self.set_tile_color` (struct :`R` 0.060958 :`G` 0.875459 :`B` 1.0 :`A` 1.0) (`self.DefaultTileTexture`)))
    (:`NewEnumerator7`
      ;[1 1 1] 友方法术影响目标
      (`self.set_tile_color` (struct :`R` 0.026912 :`G` 0.358096 :`B` 1.0 :`A` 1.0) (`self.DefaultTileTexture`)))
    (:`NewEnumerator11`
      ;[1 1 1] 中立法术可选范围
      (`self.set_tile_color` (struct :`R` 0.022554 :`G` 0.778287 :`B` 1.0 :`A` 1.0) (`self.DefaultTileTexture`)))
    (:`NewEnumerator12`
      ;[1 1 1] 中立法术选中目标
      (`self.set_tile_color` (struct :`G` 0.623002 :`B` 1.0 :`A` 1.0) (`self.DefaultTileTexture`)))
    (:`NewEnumerator13`
      ;[1 1 1] 中立法术 影响目标
      (`self.set_tile_color` (struct :`G` 0.448472 :`B` 1.0 :`A` 1.0) (`self.DefaultTileTexture`)))
    (:`NewEnumerator14`
      (`self.set_tile_color` (struct :`G` 0.68 :`B` 0.68 :`A` 1.0) (`self.DefaultTileTexture`)))
    (:`NewEnumerator15`
      (`self.set_tile_color` (struct :`R` 0.925 :`G` 0.925 :`B` 0.925 :`A` 1.0) (`self.DefaultTileTexture`)))))

(fn `set_tile_color`
  (params (color :type "LinearColor Structure") (Texture :type "Texture Object Reference"))
  (bind _dynamicmaterial (`self.DynamicMaterial`)
    (:`then`
      (`MaterialInstanceDynamic.SetVectorParameterValue` _dynamicmaterial "BaseColor" color)
      (`MaterialInstanceDynamic.SetTextureParameterValue` _dynamicmaterial "TextureSampleParameter2D" Texture))
    (:`else`)))

(fn `SetAiCacheScore`
  (params (dir :type Integer) (Score :type "Float (double-precision)"))
  (`KismetArrayLibrary.Array_Set` (`self.SimpleScoreList`) dir Score true))

(fn `swep_creature`
  (params (creaute :type "Object Object Reference"))
  (`/Engine/EditorBlueprintResources/StandardMacros.IsValid` (`self.get_creature`)
    (:`Is Valid`
      (`self.set_tile` (`self.get_creature`) null)
      (`self.set_tile` creaute self))))

(fn `UpdateAiCacheScore`
  (for _index (range 6)
    (`KismetArrayLibrary.Array_Set` (`self.SimpleScoreList`) _index -1.0 true)))

(fn `UserConstructionScript`
  (bind _outactors (`GameplayStatics.GetAllActorsOfClass` "/Game/Blueprint/Scene/HeroLevel.HeroLevel_C"))
  (set `self.HeroLevel` (`KismetArrayLibrary.Array_Get` _outactors))
  (bind _returnvalue (`PrimitiveComponent.CreateDynamicMaterialInstance` (`self.StaticMesh`) 0 "/Game/Mannequin/Character/Creature3/DyMaterial.DyMaterial"))
  (set `self.DynamicMaterial` _returnvalue)
  (`self.set_state` "NewEnumerator4"))