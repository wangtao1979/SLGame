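; HeroLevel is a hex-grid map actor that owns the tile list and saves and restores tiles, transform and scene objects through serialization data.
; Index/XY conversion and six-direction, row-parity offset math provide neighbour lookup.
; A layered BFS over tile edges, with optional passability checks, sends each step's tiles and cached parent paths to a hook that can abort it.
; Helpers compute region outline edge transforms and find tiles by location or type.
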(event EventBeginPlay)

(event EventActorBeginOverlap
  (params (OtherActor :type Actor%20Object%20Reference)))

(event EventTick
  (params (DeltaSeconds :type Float%20%28single-precision%29)))

(fn ConstructionScript)

(fn Serializationto
  (Variables|Default|SetSerializationData (Utilities|Struct|MakeSceneData (.tile (Variables|Default|GetSerializationData)) (.scenename (Variables|Default|GetSerializationData)) (Transformation|GetActorTransform) (Variables|Default|GetGridSizeY) (Variables|Default|GetGridSizeX) (.herosceneobjects (Variables|Default|GetSerializationData)) ""))
  (for _array_element (Variables|Default|GetTileList)
    (bind _newparam (Default|Serializationto _array_element))
    (Utilities|Array|Add (.tile (Variables|Default|GetSerializationData)) _newparam))
  (return (Variables|Default|GetSerializationData)))

(fn Serializationfrom
  (bind _serializationdata (Variables|Default|GetSerializationData))
  (Variables|Default|SetGridSizeX (.gridsizex _serializationdata))
  (Variables|Default|SetGridSizeY (.gridsizey _serializationdata))
  (Transformation|SetActorTransform (.transform _serializationdata))
  (for (_array_element _array_index) (.tile _serializationdata)
    (bind _returnvalue (Game|SpawnActorfromClass "/Game/Blueprint/Scene/Tile.Tile_C" (Math|Transform|MakeTransform "0, 0, 0") "Undefined" 0 0))
    (Variables|/Game/Blueprint/Scene/Tile.Tile_C|SetIndexInMap _returnvalue _array_index)
    (Utilities|Array|Add (Variables|Default|GetTileList) _returnvalue)
    (Default|Serializationfrom _returnvalue _array_element self))
  (for _array_element_2 (.herosceneobjects _serializationdata)
    (Game|SpawnActorfromClass (.objclass _array_element_2) (.transform _array_element_2) "AlwaysSpawn" 0 0))
  (Default|CallSpawnTileEnd self)
  (Default|CallCompleted))

(fn ResetState
  (for _array_element (Variables|Default|GetTileList)
    (Default|SetState _array_element "NewEnumerator4")))

(fn GetTilebyIndex
  (params (Index :type Integer))
  (return (Utilities|Array|Get(acopy) (Variables|Default|GetTileList) Index)))

(fn MathMoveto
  (params (X :type Integer) (Y :type Integer) (Dir :type Integer))
  (bind (_localy _returnvalue) (|MoveToDir0_2))
  (bind (_returnvalue_2 _returnvalue2) (|MoveToDir5_2))
  (bind (_returnvalue_3 _returnvalue2_2) (|MoveToDir1_2))
  (bind (_returnvalue_4 _returnvalue2_3) (|MoveToDir2_2))
  (bind (_returnvalue_5 _localy_2) (|MoveToDir3_2))
  (bind (_returnvalue_6 _returnvalue2_4) (|MoveToDir4_2))
  (Utilities|FlowControl|Sequence
    (:then_0
      (LocalVariables|SetLocalX X))
    (:then_1
      (LocalVariables|SetLocalY Y))
    (:then_2
      (switch int Dir
        (:0
          (return _returnvalue _localy))
        (:1
          (return _returnvalue_3 _returnvalue2_2))
        (:2
          (return _returnvalue_4 _returnvalue2_3))
        (:3
          (return _returnvalue_5 _localy_2))
        (:4
          (return _returnvalue_6 _returnvalue2_4))
        (:5
          (return _returnvalue2 _returnvalue_2))))))

(fn XYtoIndex
  (params (X :type Integer) (Y :type Integer))
  (if (or (or (>= X (Variables|Default|GetGridSizeX)) (< X 0)) (or (< Y 0) (>= Y (Variables|Default|GetGridSizeY))))
    (return -1)
    (else
      (return (+ X (* Y (Variables|Default|GetGridSizeX)))))))

(fn IndextoXY
  (params (Index :type Integer))
  (return (|(Index%{E939E845-4612-AF22-D240-9885D759C1D0}) Index) (|(Index/{E939E845-4612-AF22-D240-9885D759C1D0}) Index)))

(fn Bfs
  (params (SearchStep :type Integer) (CheckPassable :type Boolean) (StartTile :type Tile%20Object%20Reference) (StepHook :type BFS%20Step%20Hook%20Interface))
  (LocalVariables|SetBfsTotalStep SearchStep)
  (LocalVariables|SetBfsCheckPassable CheckPassable)
  (Utilities|Array|Clear (LocalVariables|GetBfsCurrQueueWithLevel))
  (Utilities|Array|Add (LocalVariables|GetBfsCurrQueueWithLevel) StartTile)
  (Utilities|Array|Add (LocalVariables|GetBfsCurrQueue) StartTile)
  (Utilities|Array|Add (LocalVariables|GetBfsKnownSet) StartTile)
  (Utilities|Array|SetArrayElem (LocalVariables|GetBfsPathCache) (Variables|/Game/Blueprint/Scene/Tile.Tile_C|GetIndexInMap StartTile) -1 true)
  (while (not (or (== (Utilities|Array|Length (LocalVariables|GetBfsCurrQueueWithLevel)) 0) (> (LocalVariables|GetBfsCurrStep) (LocalVariables|GetBfsTotalStep))))
    (Utilities|FlowControl|Sequence
      (:then_0
        (for _array_element (LocalVariables|GetBfsCurrQueueWithLevel)
          (Utilities|Array|Add (LocalVariables|GetBfsHookData) (Utilities|Struct|MakeTileWithPath _array_element (CallFunction|GetPathfromCache _array_element (LocalVariables|GetBfsPathCache)))))
        (bind _searchmore (Class|BFSStepHook|BfsStepHook(Message) (Utilities|ToObject(Interface) StepHook) (LocalVariables|GetBfsHookData) (LocalVariables|GetBfsCurrStep)))
        (if (not _searchmore)
          (return)))
      (:then_1
        (Utilities|Array|Clear (LocalVariables|GetBfsCurrQueueWithLevel)))
      (:then_2
        (for _array_element_2 (LocalVariables|GetBfsCurrQueue)
          (bind _output_get (LocalVariables|SetBfsTempParent _array_element_2))
          (for _array_element_3 (Variables|/Game/Blueprint/Scene/Tile.Tile_C|GetEdge _output_get)
            (bind _output_get_2 (LocalVariables|SetBfsNewTile _array_element_3))
            (Utilities|IsValid _output_get_2
              (:Is%20Valid
                (if (not (Utilities|Array|ContainsItem (LocalVariables|GetBfsKnownSet) (LocalVariables|GetBfsNewTile)))
                  (Utilities|Array|Add (LocalVariables|GetBfsKnownSet) (LocalVariables|GetBfsNewTile))
                  (Utilities|Array|Add (LocalVariables|GetBfsCurrQueueWithLevel) (LocalVariables|GetBfsNewTile))
                  (Utilities|Array|SetArrayElem (LocalVariables|GetBfsPathCache) (Variables|/Game/Blueprint/Scene/Tile.Tile_C|GetIndexInMap (LocalVariables|GetBfsNewTile)) (Variables|/Game/Blueprint/Scene/Tile.Tile_C|GetIndexInMap (LocalVariables|GetBfsTempParent)) true)
                  (if (LocalVariables|GetBfsCheckPassable)
                    (if (Default|ControlCreatureCanPass (LocalVariables|GetBfsNewTile))
                      (Utilities|Array|Add (LocalVariables|GetBfsTempQueue) (LocalVariables|GetBfsNewTile) :!label _label))
                    (else
                      (goto _label))))))))
        (LocalVariables|SetBfsCurrQueue (LocalVariables|GetBfsTempQueue))
        (Utilities|Array|Clear (LocalVariables|GetBfsTempQueue))
        (Math|Integer|IncrementInt (LocalVariables|GetBfsCurrStep)
          (:%20%20
            (Utilities|Array|Clear (LocalVariables|GetBfsHookData)))))))
  (return))

(fn GetPathfromCache
  (params (DstTile :type Tile%20Object%20Reference) (Cache :type Array%20of%20Integers))
  (LocalVariables|SetPathCache Cache)
  (LocalVariables|SetCurrIndex (Variables|/Game/Blueprint/Scene/Tile.Tile_C|GetIndexInMap DstTile))
  (while (!= (LocalVariables|GetCurrIndex) -1)
    (Utilities|Array|Insert (LocalVariables|GetResultPath) (CallFunction|GetTilebyIndex (LocalVariables|GetCurrIndex)))
    (LocalVariables|SetCurrIndex (Utilities|Array|Get(acopy) (LocalVariables|GetPathCache) (LocalVariables|GetCurrIndex))))
  (return (LocalVariables|GetResultPath)))

(fn GetMaskOutline
  (params (TileList :type Array%20of%20Tile%20Object%20References))
  (bind _output_get (LocalVariables|SetLocalTileList TileList))
  (for _array_element _output_get
    (bind _output_get_2 (LocalVariables|SetLocalParentTile _array_element))
    (bind (_x _y) (CallFunction|IndextoXY (Variables|/Game/Blueprint/Scene/Tile.Tile_C|GetIndexInMap _output_get_2)))
    (for _index (range 0 5)
      (bind _output_get_3 (LocalVariables|SetLocalDir _index))
      (bind (_newx _newy) (CallFunction|MathMoveto _x _y _output_get_3))
      (bind _index_2 (CallFunction|XYtoIndex _newx _newy))
      (bind _output_get_4 (LocalVariables|SetLocalIndex _index_2))
      (if (== _output_get_4 -1)
        (bind _trans (CallFunction|GetTileEdgeTrans (LocalVariables|GetLocalParentTile) (LocalVariables|GetLocalDir) :!label _label))
        (Utilities|Array|Add (LocalVariables|GetLocalResult) _trans)
        (elif (not (Utilities|Array|ContainsItem (LocalVariables|GetLocalTileList) (CallFunction|GetTilebyIndex (LocalVariables|GetLocalIndex))))
          (goto _label)))))
  (return (LocalVariables|GetLocalResult)))

(fn GetTileEdgeTrans
  (params (Tile :type Tile%20Object%20Reference) (Dir :type Integer))
  (bind _staticmesh (Variables|/Game/Blueprint/Scene/Tile.Tile_C|GetStaticMesh Tile))
  (bind _defaultsceneroot (Variables|/Game/Blueprint/Scene/Tile.Tile_C|GetDefaultSceneRoot Tile))
  (bind (_min _max) (Components|StaticMesh|GetLocalBounds _staticmesh))
  (bind _returnvalue (Transformation|GetWorldRotation _defaultsceneroot))
  (bind _output_get (LocalVariables|SetNewLocalVar_0 (Math|Rotator|MakeRotator (.roll _returnvalue) (.pitch _returnvalue) (+ (.yaw _returnvalue) (Math|Conversions|ToFloat(Integer) (* (Math|Integer|%(Integer) (- Dir 3) 6) 60))))))
  (return (Math|Transform|MakeTransform (+ (Transformation|GetWorldLocation (Variables|/Game/Blueprint/Scene/Tile.Tile_C|GetDefaultSceneRoot Tile)) (* (Math|Vector|Normalize (Math|Vector|GetForwardVector _output_get)) (* (/ (- (.x _max) (.x _min)) 2.0) (.x (.scale (Transformation|GetActorTransform)))))) _output_get (.scale (Transformation|GetActorTransform)))))

(fn LocationtoIndex
  (params (location :type Vector))
  (for _array_element (Variables|Default|GetTileList)
    (LocalVariables|Setcur_distance (Math|Vector|VectorLengthSquared (- location (Transformation|GetActorLocation _array_element))))
    (if (or (> (LocalVariables|Getmin_distance) (LocalVariables|Getcur_distance)) (not (Utilities|IsValid (LocalVariables|Getmin_tile))))
      (LocalVariables|Setmin_tile _array_element)
      (LocalVariables|Setmin_distance (LocalVariables|Getcur_distance))))
  (return (Default|GetTileIndex (LocalVariables|Getmin_tile))))

(fn GetAllTileList
  (return (Variables|Default|GetTileList)))

(fn GetTilebyType
  (params (type :type TileTypeEnum%20Enum))
  (for _array_element (Variables|Default|GetTileList)
    (if (Utilities|Enum|Equal(Enum) type (Default|GetType _array_element))
      (Utilities|Array|Add (LocalVariables|Getmatch_tile_list) _array_element)))
  (return (LocalVariables|Getmatch_tile_list)))