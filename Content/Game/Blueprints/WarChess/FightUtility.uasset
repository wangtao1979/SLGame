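; Utility function library for WarChess fights, covering targeting rules, attack matchups and creature spawning.
; Tile validation filters by target type using occupancy, life state and faction-based friend/enemy checks, with an optional simulated caster tile.
; Attack results come from the defence-minus-attack type difference, wrapped by enum size.
; Spawn helpers create creatures from serialized data at a transform or on a tile, falling back to tile zero for invalid saved indices.
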(fn `get_attack_result`
  (params (cast :type "Object Object Reference") (target :type "Object Object Reference"))
  (returns (result :type "/Game/Game/Blueprints/WarChess/Fight/Computer/AttackResult Enum"))
  (locals (value :type Byte))
  (bind _returnvalue (- (`self.get_defance_type` target) (`self.get_attack_type` cast)))
  (bind _returnvalue_2 (`KismetMathLibrary.Conv_IntToByte` (enumcount `/Game/Game/Blueprints/WarChess/Fight/Computer/AttackResult`)))
  (return (cast `/Game/Game/Blueprints/WarChess/Fight/Computer/AttackResult` (select `bool` (>= _returnvalue _returnvalue_2) :`false` _returnvalue :`true` (+ _returnvalue _returnvalue_2)))))

(fn `get_max_ranger`
  (returns (max_ranger :type Integer))
  (return 16))

(fn `is_enemy`
  (params (creature1 :type "Object Object Reference") (creature2 :type "Object Object Reference"))
  (returns (is_enemy :type Boolean))
  (if (and (`KismetSystemLibrary.IsValid` creature1) (`KismetSystemLibrary.IsValid` creature2))
    (return (`|EnumInequality` (`self.get_faction` creature1) (`self.get_faction` creature2)))
    (else
      (return false))))

(fn `is_friend`
  (params (creature1 :type "Object Object Reference") (creature2 :type "Object Object Reference"))
  (returns (is_friend :type Boolean))
  (if (and (`KismetSystemLibrary.IsValid` creature1) (`KismetSystemLibrary.IsValid` creature2))
    (return (`|EnumEquality` (`self.get_faction` creature1) (`self.get_faction` creature2)))
    (else
      (return false))))

(fn `is_valid_tile`
  (params (caster :type "Object Object Reference") (target :type "/Game/Blueprint/Scene/Tile Object Reference") (type :type "/Game/Game/Blueprints/WarChess/Skill/Data/SkillEffectTraget Enum") (simula :type "/Game/Blueprint/Scene/Tile Object Reference"))
  (returns (is_effect :type Boolean))
  (locals (tile_creature :type "Object Object Reference") (is_exist_creature :type Boolean) (is_alive :type Boolean) (cast_creature_tile :type "/Game/Blueprint/Scene/Tile Object Reference") (target_tile :type "/Game/Blueprint/Scene/Tile Object Reference") (cast_creature :type "Object Object Reference") (real_caster_tile :type "/Game/Blueprint/Scene/Tile Object Reference"))
  (bind _is_enemy (`self.is_enemy` null))
  (bind _is_friend (`self.is_friend` null))
  (set `local.cast_creature` null)
  (bind _output_get (set `local.real_caster_tile` (`self.get_tile`)))
  (set `local.target_tile` target)
  (set `local.cast_creature_tile` (select `bool` (`KismetSystemLibrary.IsValid` simula) :`false` _output_get :`true` simula))
  (if (and (!= (`local.cast_creature_tile`) (`local.real_caster_tile`)) (`KismetSystemLibrary.IsValid` (`local.real_caster_tile`)))
    (if (== (`local.target_tile`) (`local.cast_creature_tile`))
      (set `local.tile_creature` null)
      (elif (== (`local.target_tile`) (`local.real_caster_tile`))
        (set `local.tile_creature` null)
        (else
          (set `local.tile_creature` null :!label _label))))
    (else
      (goto _label)))
  (if (`KismetSystemLibrary.IsValid` null)
    (set `local.is_exist_creature` true)
    (set `local.is_alive` (`self.is_alive`)))
  (switch `/Game/Game/Blueprints/WarChess/Skill/Data/SkillEffectTraget` type
    (:`NewEnumerator2`
      (return true))
    (:`NewEnumerator0`
      (return (and (`local.is_exist_creature`) _is_enemy (`local.is_alive`))))
    (:`NewEnumerator1`
      (return (and (`local.is_exist_creature`) _is_friend (`local.is_alive`))))
    (:`NewEnumerator3`
      (return (not (`local.is_exist_creature`))))
    (:`NewEnumerator4`
      (return (and (`local.is_exist_creature`) (`local.is_alive`))))
    (:`NewEnumerator5`
      (return (and (`local.is_exist_creature`) _is_friend (not (`local.is_alive`)))))
    (:`NewEnumerator6`
      (return (and (`local.is_exist_creature`) _is_enemy (not (`local.is_alive`)))))
    (:`NewEnumerator7`
      (return (and (`local.is_exist_creature`) (not (`local.is_alive`)))))
    (:`NewEnumerator8`
      (return (== (`local.target_tile`) (`local.cast_creature_tile`))))))

(fn `spawn_careture_to_pos`
  (params (creature_data :type "/Game/Game/Blueprints/WarChess/Unit/Data/MulCreatureData Structure") (creature_type :type "Object Class Reference") (transfrome :type "Transform Structure"))
  (returns (creature :type "Object Object Reference"))
  (bind _returnvalue (`|SpawnActorFromClass` (select `bool` (`KismetSystemLibrary.IsValidClass` creature_type) :!type "Actor Class Reference") transfrome "Undefined" "OverrideRootScale"))
  (`self.SerializationFrom` _returnvalue creature_data)
  (`Actor.K2_SetActorTransform` _returnvalue transfrome false false)
  (return _returnvalue))

(fn `spawn_creature`
  (params (creature_data :type "/Game/Game/Blueprints/WarChess/Unit/Data/MulCreatureData Structure") (creature_type :type "Object Class Reference") (faction :type "/Game/Game/Blueprints/WarChess/Fight/Team/FactionEnum Enum"))
  (returns (creature :type "Object Object Reference"))
  (locals (tile :type "/Game/Blueprint/Scene/Tile Object Reference"))
  (bind _output_get (set `local.tile` (`/Game/Blueprint/Scene/HeroLevel.GetTileByIndex` (`self.get_hero_level` (`self.get_fight_game_mode` null)) (`.tile_index_25_1B76483F49AB8FF3E52E4AAFFE834D2F` (break `/Game/Game/Blueprints/WarChess/Unit/Data/CreatureData` (`KismetArrayLibrary.Array_Get` (`.data_3_5525F4DD440256C69AB3CE95D205B539` (break `/Game/Game/Blueprints/WarChess/Unit/Data/MulCreatureData` creature_data))))))))
  (if (not (`KismetSystemLibrary.IsValid` _output_get))
    (bind _output_get_2 (set `local.tile` (`/Game/Blueprint/Scene/HeroLevel.GetTileByIndex` (`self.get_hero_level` (`self.get_fight_game_mode` null)) 0))))
  (bind _creature (`self.spawn_creature_to_tile` creature_data _output_get_2 creature_type faction))
  (return _creature))

(fn `spawn_creature_to_tile`
  (params (crature_data :type "/Game/Game/Blueprints/WarChess/Unit/Data/MulCreatureData Structure") (tile :type "/Game/Blueprint/Scene/Tile Object Reference") (creature_type :type "Object Class Reference") (faction :type "/Game/Game/Blueprints/WarChess/Fight/Team/FactionEnum Enum"))
  (returns (creature :type "Object Object Reference"))
  (locals (target_tile :type "/Game/Blueprint/Scene/Tile Object Reference"))
  (bind _output_get (set `local.target_tile` tile))
  (if (`KismetSystemLibrary.IsValid` _output_get)
    (bind _returnvalue (`|SpawnActorFromClass` (select `bool` (`KismetSystemLibrary.IsValidClass` creature_type) :!type "Actor Class Reference") (`KismetMathLibrary.MakeTransform` (0.0 0.0 0.0)) "AlwaysSpawn" "OverrideRootScale"))
    (`self.SerializationFrom` _returnvalue crature_data)
    (`self.set_faction` _returnvalue faction)
    (`self.stand_on_tile` _returnvalue (`local.target_tile`))
    (return _returnvalue)
    (else
      (return null))))