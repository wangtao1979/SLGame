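; ArsenalCreature is a War Chess Blueprint that links a creature to the factory it comes from, judging by its BindCreature inputs.
; BindCreature assigns the Creature and Factory variables, though the graph shows them set to None.
; GetReportData is an empty stub; disconnected leftover nodes read the creature's HP scale and would pick a state based on whether it is below full.
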(fn `bind_creature`
  (params (creature :type "Object Object Reference") (factory :type "Object Object Reference"))
  (set `self.creature` null)
  (set `self.factory` null))

(fn `get_report_data`
  (returns (report_data :type " Structure")))