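; Game mode for turn-based tile battles, running a fight from scene loading and intro movie through PVE/PVP tactics setup to the result screen.
; SceneLoader builds the level, arsenal troops spawn as draggable player creatures, and TurnManager drives turns and camera follow on moves and casts.
; FightRecorder records fights or replays them from saved random data and actions.
; Live results report stars and troops to the server, with records for PVP.
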(event `self.ReceiveBeginPlay`
  (set `self.troops_manager` (`self.get_troops_manager` (`self.get_hero_game_instance`)))
  (set `self.network` (`self.get_network` (`self.get_hero_game_instance`)))
  (`self.load_configer`))

(event `StartFight`
  ;[1 1 1] 开始战斗
  (`self.InitRecrod`)
  (`self.BindCamera`)
  (`/Game/Game/Blueprints/WarChess/Fight/turn/TurnManager.start_game` (`self.TurnManager`))
  (add `/Game/Game/Blueprints/WarChess/Fight/turn/TurnManager.NextTurn` (`self.TurnManager`) (delegate `OnNextTurn`))
  (`self.FightStart`))

(event `OnNextTurn`
  (params (turn_index :type Integer))
  ;[1 1 1] 开始战斗
  (bind _returnvalue (`|CreateWidget` null))
  (`UserWidget.AddToViewport` _returnvalue 0))

(event `BindCamera`
  ;[1 1 1] 镜头处理
  (add `/Game/Game/Blueprints/WarChess/Fight/turn/TurnManager.Next` (`self.TurnManager`) (delegate `OnSwitchCamera`))
  (add `/Game/Game/Blueprints/WarChess/Fight/turn/TurnManager.Insert` (`self.TurnManager`) (delegate `OnBindCreatureCamera`))
  (for _array_element (`/Game/Game/Blueprints/WarChess/Fight/turn/TurnManager.get_all_creature_list` (`self.TurnManager`))
    (bind _ascreature (cast `` _array_element))
    (`self.OnBindCreatureCamera` _ascreature)))

(event `StartTacitcs`
  ;[1 1 1] 开始进行战术配置
  (switch `|SwitchEnum` (`self.get_cur_level_type` (`self.get_hero_game_instance`))
    (:`NewEnumerator0`
      (bind _returnvalue (`|CreateWidget` null))
      (`UserWidget.AddToViewport` _returnvalue 0))
    (:`NewEnumerator1`
      (bind _returnvalue_2 (`|CreateWidget` null))
      (`UserWidget.AddToViewport` _returnvalue_2 0))))

(event `OnBindCreatureCamera`
  (params (creature :type "Object Object Reference"))
  ;[1 1 1] 镜头处理
  (add `self.StartMove` creature (delegate `OnLockCamera`))
  (add `self.EndMove` creature (delegate `OnUnLockCamera`))
  (add `self.Cast` creature (delegate `SetCameraTwoTargetCenter`)))

(event `OnSwitchCamera`
  (params (creature :type "Object Object Reference"))
  ;[1 1 1] 镜头处理
  (`self.SmoothMoveToBySpeed` (`self.get_hero_spawn`) 20000.0 (`self.K2_GetActorLocation` creature) (`SpringArmComponent.TargetArmLength` (`/Game/Game/Blueprints/WarChess/BPHeroGameMode.SpringArm` (`self.get_hero_spawn`)))))

(event `OnUnLockCamera`
  ;[1 1 1] 镜头处理
  (`self.KeepLookAt` (`self.get_hero_spawn`) null))

(event `SetCameraTwoTargetCenter` :!signature `self.Cast`
  (params (skill :type "/Game/Game/Blueprints/WarChess/Skill/Logic/Skill Object Reference") (cast_tile :type "/Game/Blueprint/Scene/Tile Object Reference"))
  ;[1 1 1] 镜头处理
  (add `self.MoveEnd` (`self.get_hero_spawn`) (delegate `RestoreCamera`))
  (set `self.ArmLengthBk` (`SpringArmComponent.TargetArmLength` (`/Game/Game/Blueprints/WarChess/BPHeroGameMode.SpringArm` (`self.get_hero_spawn`))))
  (bind (_moveto _armlength) (`self.GetLerpInfor` (`self.get_hero_spawn`) (`self.get_tile` (`/Game/Game/Blueprints/WarChess/Fight/turn/TurnManager.get_control_creature` (`self.TurnManager`))) cast_tile))
  (`self.SmoothMoveTo ` (`self.get_hero_spawn`) _moveto _armlength))

(event `OnLockCamera`
  ;[1 1 1] 镜头处理
  (`self.KeepLookAt` (`self.get_hero_spawn`) (`/Game/Game/Blueprints/WarChess/Fight/turn/TurnManager.get_control_creature` (`self.get_turn_manager`))))

(event `RestoreCamera`
  ;[1 1 1] 镜头处理
  (remove `self.MoveEnd` (`self.get_hero_spawn`) (delegate `RestoreCamera`))
  (set `SpringArmComponent.TargetArmLength` (`self.ArmLengthBk`) (`/Game/Game/Blueprints/WarChess/BPHeroGameMode.SpringArm` (`self.get_hero_spawn`))))

(event `EndTacitcs`
  ;[1 1 1] 结束战斗配置
  (`self.CreatureLoaded`)
  (for _array_element (`/Game/Game/Blueprints/WarChess/Fight/Team/Team.get_all_member` (`self.PlayerTeam`))
    (`self.disable_drag_drop` _array_element))
  (bind _returnvalue (`|CreateWidget` null))
  (`UserWidget.AddToViewport` _returnvalue 0)
  (`self.TacitcsEnd`))

(event `self.SceneLoader.SceneComplete`
  ;[1 1 1] 场景装载完成
  (`self.SceneLoaded`))

(event `self.SceneLoader.InitHeroLevel`
  (params (herolevel :type "/Game/Blueprint/Scene/HeroLevel Object Reference"))
  ;[1 1 1] Comment
  (set `self.hero_level` (`/Game/Game/Blueprints/WarChess/BPHeroGameMode.HeroLevel` (`self.SceneLoader`))))

(event `self.TurnManager.End`
  (params (reslut :type "/Game/Game/Blueprints/WarChess/Fight/turn/FightResult Enum" :default "NewEnumerator0"))
  ;[1 1 1] 战棋战斗结束
  (`self.set_global_time` (`self.get_hero_game_instance`) 0.25)
  (`KismetSystemLibrary.Delay` 1.0)
  (`self.set_global_time` (`self.get_hero_game_instance`) 1.0)
  (`self.stop_all_amient_sound`)
  (`self.EndFight` reslut)
  (switch `/Game/Game/Blueprints/WarChess/Fight/turn/FightResult` reslut
    (:`NewEnumerator0`
      (bind _returnvalue (`|CreateWidget` null))
      (`UserWidget.AddToViewport` _returnvalue 0))
    (:`NewEnumerator1`
      (bind _returnvalue_2 (`|CreateWidget` null))
      (`UserWidget.AddToViewport` _returnvalue_2 0))))

(event `self.ReceiveTick`
  (params (DeltaSeconds :type "Float (single-precision)"))
  ;[1 1 1] 计算当前帧
  (`self.on_frame` (`self.get_hero_game_instance`)))

(event `ReportFight`
  (params (reslut :type Boolean) (quit :type Boolean))
  (bind _returnvalue (select `bool` reslut :`true` (`self.count_fight_star`)))
  ;[1 1 1] 报告战斗结果
  (if (`self.is_record` (`self.get_hero_game_instance`))
    (`self.escape_to_city` (`self.get_hero_game_instance`))
    (else
      (bind _returnvalue_2 (`|GenericCreateObject` null self))
      (switch `|SwitchEnum` (`self.get_cur_level_type` (`self.get_hero_game_instance`))
        (:`NewEnumerator0`
          (`self.set_result` :`self` _returnvalue_2 :`star` _returnvalue :`level_id` (`self.get_id` (`self.get_cur_fight_level` (`self.get_levels_manager` (`self.get_hero_game_instance`)))) :`troops` (`self.count_troops_report`) :`Serialization Data Quit` quit))
        (:`NewEnumerator1`
          (`self.set_result` _returnvalue_2 _returnvalue 0 0 (`self.get_key` (`self.get_search_target` (`self.get_pvp_manager` (`self.get_hero_game_instance`)))) (`/Game/Game/Blueprints/WarChess/Fight/Record/FightRecorder.GetRecordData` (`self.FightRecorder`)) (`self.count_troops_report`) quit)))
      (`self.send_message` (`self.network`) _returnvalue_2))))

(event `StartLoadDstLevel`
  (`self.SetSeamlessTravelMidpointPause` false))

(fn `can_play_movie`
  (returns (can_play :type Boolean))
  (return true))

(fn `count_fight_star`
  (returns (star_count :type Integer))
  (locals (dead_count :type Integer))
  (for _array_element (`/Game/Game/Blueprints/WarChess/Fight/Team/Team.get_all_member` (`self.get_team` "NewEnumerator0"))
    (if (and (not (`self.is_alive` _array_element)) (not (`self.is_summoned` _array_element)))
      (`/Engine/EditorBlueprintResources/StandardMacros.IncrementInt` (`local.dead_count`))))
  (return (`KismetMathLibrary.Max` (- 3 (`local.dead_count`)))))

(fn `count_troops_report`
  (returns (troops_info :type "Array of  Structure"))
  (locals (troops_array :type "Array of  Structure"))
  (for _array_element (`self.arsenal_creature_list`)
    (`/Engine/EditorBlueprintResources/StandardMacros.IsValid` _array_element
      (:`Is Valid`
        (`KismetArrayLibrary.Array_Add` (`local.troops_array`) (`/Game/Game/Blueprints/WarChess/ArsenalCreature.get_report_data` _array_element)))))
  (return (`local.troops_array`)))

(fn `end_movie`
  (set `self.playing_matinee` null)
  (if (`self.is_record` (`self.get_hero_game_instance`))
    (bind _returnvalue (`|CreateWidget` null))
    (`UserWidget.AddToViewport` _returnvalue 0)
    (else
      (`self.StartTacitcs`)
      (`self.TitleMovieEnd`))))

(fn `escape_fight`
  (`self.escape_to_city` (`self.get_hero_game_instance`))
  (`self.send_command` (`self.network`) "EscapeFight"))

(fn `ExGetSeamlessTravelActorList`
  (params (bToEntry :type Boolean))
  (returns (ReturnValue :type "Array of Actor Object Reference"))
  (locals (NewLocalVar_0 :type "Array of Actor Object Reference"))
  (if bToEntry
    (bind _returnvalue (`|CreateWidget` null))
    (`UserWidget.AddToViewport` _returnvalue 0)
    (else
      (`WidgetLayoutLibrary.RemoveAllWidgets`)))
  (return (`local.NewLocalVar_0`)))

(fn `get_hero_level`
  (returns (hero_level :type "/Game/Blueprint/Scene/HeroLevel Object Reference"))
  (return (`self.hero_level`)))

(fn `get_recorder`
  (returns (FightRecorder :type "/Game/Game/Blueprints/WarChess/Fight/Record/FightRecorder Object Reference"))
  (return (`self.FightRecorder`)))

(fn `get_team`
  (params (faction :type "/Game/Game/Blueprints/WarChess/Fight/Team/FactionEnum Enum"))
  (returns (Team :type "/Game/Game/Blueprints/WarChess/Fight/Team/Team Object Reference"))
  (switch `/Game/Game/Blueprints/WarChess/Fight/Team/FactionEnum` faction
    (:`NewEnumerator0`
      (return (`self.PlayerTeam`)))
    (:`NewEnumerator1`
      (return (`self.EnemyTeam`)))
    (:`NewEnumerator3`
      (return null))))

(fn `GetEnemyMaster`
  (params (faction :type "/Game/Game/Blueprints/WarChess/Fight/Team/FactionEnum Enum"))
  (returns (creature :type "Object Object Reference"))
  (return (`/Game/Game/Blueprints/WarChess/Fight/turn/TurnManager.GetEnemyMaster` (`self.TurnManager`) faction)))

(fn `init_exist_creature`
  (locals (aresnal_list :type "Array of Object Object Reference") (cur_arenal :type "Object Object Reference") (tile_list :type "Array of /Game/Blueprint/Scene/Tile Object Reference") (index :type Integer) (player_dir :type Integer :default 0))
  (set `local.player_dir` 3)
  (set `local.tile_list` (`/Game/Blueprint/Scene/HeroLevel.get_tile_by_type` (`self.hero_level`) "NewEnumerator8"))
  (bind _output_get (set `local.aresnal_list` (`self.get_all_asenal` (`self.troops_manager`))))
  (for _array_element _output_get
    (bind _output_get_2 (set `local.cur_arenal` _array_element))
    (if (`KismetSystemLibrary.IsValid` _output_get_2)
      (if (`self.can_fight` (`local.cur_arenal`))
        (bind _creature (`/Game/Game/Blueprints/WarChess/FightUtility.spawn_creature_to_tile` (`self.get_mul_creature_data` (`self.get_exist_troops` (`local.cur_arenal`))) (`KismetArrayLibrary.Array_Get` (`local.tile_list`) (`local.index`)) null "NewEnumerator0"))
        (`self.enable_drag_drop` _creature (`|MakeArray` "NewEnumerator4" "NewEnumerator8" :!type "/Game/Game/Blueprints/WarChess/Scene/Data/TileTypeEnum Enum"))
        (`self.updatedir` _creature (`local.player_dir`))
        (bind _returnvalue (`|GenericCreateObject` "/Game/Game/Blueprints/WarChess/ArsenalCreature.ArsenalCreature_C" self))
        (`/Game/Game/Blueprints/WarChess/ArsenalCreature.bind_creature` _returnvalue _creature (`local.cur_arenal`))
        (`KismetArrayLibrary.Array_Add` (`self.arsenal_creature_list`) _returnvalue)
        (`/Engine/EditorBlueprintResources/StandardMacros.IncrementInt` (`local.index`)))))
  (`KismetArrayLibrary.Array_Append` (`local.tile_list`) (`/Game/Blueprint/Scene/HeroLevel.get_tile_by_type` (`self.hero_level`) "NewEnumerator4"))
  (for _array_element_2 (`local.tile_list`)
    (switch `/Game/Game/Blueprints/WarChess/Scene/Data/TileTypeEnum` (`/Game/Blueprint/Scene/Tile.get_type` _array_element_2)
      (:`NewEnumerator4`
        _)
      (:`NewEnumerator8`
        _))
    (`/Game/Blueprint/Scene/Tile.set_state` _array_element_2 "NewEnumerator0")))

(fn `InitRecordTroops`
  (bind (_random _fightactionlist _attacktroops _defencetroops _attackplayer _defenceplayer _scene _scenedata _card_id _card_level _card_skill) (break `` (`/Game/Game/Blueprints/WarChess/BPHeroGameMode.SerializationData` (`self.get_fight_record` (`self.get_hero_game_instance`)))))
  (`/Game/Game/Blueprints/WarChess/Fight/Record/FightRecorder.SetRecorodData` (`self.FightRecorder`) _random _fightactionlist)
  (`self.SetRandomData` (`self.get_random_generator` (`self.get_hero_game_instance`)) _random)
  (`/Game/Game/Blueprints/WarChess/Fight/Record/FightRecorder.SetHeroCard` (`self.FightRecorder`) _card_skill))

(fn `InitRecrod`
  (if (`self.is_record` (`self.get_hero_game_instance`))
    (`/Game/Game/Blueprints/WarChess/Fight/Record/FightRecorder.PlayRecord` (`self.FightRecorder`))
    (else
      (`/Game/Game/Blueprints/WarChess/Fight/Record/FightRecorder.StartRecord` (`self.FightRecorder`)))))

(fn `load_configer`
  (locals (game_instance :type "Object Object Reference"))
  (bind _output_get (set `local.game_instance` (`self.get_hero_game_instance`)))
  (if (`self.is_record` _output_get)
    (`self.LoadConfiger` (`self.SceneLoader`) (`.SceneData_39_887BAB2845A0638C5A4447BE880BFB2F` (break `` (`/Game/Game/Blueprints/WarChess/BPHeroGameMode.SerializationData` (`self.get_fight_record` (`local.game_instance`))))))
    (`self.InitRecordTroops`)
    (`self.CreatureLoaded`)
    (else
      (`self.LoadConfiger` (`self.SceneLoader`) (`.scene_2_A0A6C34F415F2A20F1FD44AFB3B989E9` (break `` (`/Game/Game/Blueprints/WarChess/BPHeroGameMode.SerializationData` (`self.get_fight_level_data` (`local.game_instance`))))))
      (`self.init_exist_creature`))))

(fn `play_movie`
  (params (matinee :type "MatineeActor Object Reference"))
  (bind _output_get (set `self.playing_matinee` matinee))
  (`MatineeActor.Play` _output_get))

(fn `stop_all_amient_sound`
  ;[1 1 1] 停止环境音
  (bind _outactors (`GameplayStatics.GetAllActorsOfClass` "/Script/Engine.AmbientSound"))
  (for _array_element _outactors
    (`AudioComponent.Stop` (`AmbientSound.AudioComponent` _array_element))))

(fn `stop_movie`
  (bind _playing_matinee (`self.playing_matinee`)
    (:`then`
      (`MatineeActor.Stop` _playing_matinee)
      (`self.end_movie`))
    (:`else`)))

(fn `UserConstructionScript`)